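; BP_SparkCharacter_AI_OrcArcher is the AI orc archer character that shoots arrows at its blackboard target.
; Its construction script attaches the bow mesh to the left hand socket.
; The FireArrow event spawns an orc arrow projectile at a mesh socket and plays a bow sound.
; The arrow is aimed at the target's capsule center of mass for characters, otherwise at the actor location.
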(event `FireArrow`
  (bind _returnvalue (`BlackboardComponent.GetValueAsObject` (`AIBlueprintHelperLibrary.GetBlackboard` null) "Target"))
  (bind _location (.location (`SceneComponent.GetSocketTransform` (`self.Mesh`) "FireArrowSocket" "RTS_World")))
  (bind (_ascharacter _bsuccess) (cast `Character` _returnvalue :!pure true))
  ;[1 1 1] Fire arrow!
  (`|SpawnActorFromClass` "/Game/Gameplay/Combat/BP_Projectile_OrcArrow.BP_Projectile_OrcArrow_C" (`KismetMathLibrary.MakeTransform` _location (`KismetMathLibrary.FindLookAtRotation` _location (`KismetMathLibrary.SelectVector` (`PrimitiveComponent.GetCenterOfMass` (`Character.CapsuleComponent` _ascharacter) "None") (`self.K2_GetActorLocation` (cast `Actor` _returnvalue :!pure true)) _bsuccess))) "AlwaysSpawn" "OverrideRootScale" self self)
  (`GameplayStatics.PlaySoundAtLocation` "/Game/Characters/Orc/Sound/SC_Bow_Fire.SC_Bow_Fire" (`self.K2_GetActorLocation`) (struct) 1.0 1.0 0.0 null null null))

(fn `UserConstructionScript`
  (`parent.UserConstructionScript`)
  ;[1 1 1] Attach the bow
  (`SceneComponent.K2_AttachToComponent` (`self.ArcherBowMesh`) (`self.Mesh`) "LeftHandSocket" "SnapToTarget" "KeepRelative" "KeepRelative" true))