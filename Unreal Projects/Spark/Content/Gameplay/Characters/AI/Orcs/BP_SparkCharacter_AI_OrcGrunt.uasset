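; Orc grunt AI character that fights the player with a one-handed axe attack and a shield bash.
; The construction script snaps the axe and shield to the hand sockets and enlarges the shield.
; Each attack event sphere-traces forward from its hand socket for pawns, using a reset DoOnce to limit damage to one hit.
; The bash also stops the player's charge and launches them away along the grunt's facing.
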(event `Grunt1hAttack`
  (bind _returnvalue (`SceneComponent.GetSocketLocation` (`self.Mesh`) "RightHandSocket"))
  ;[1 1 1] One handed attack
  (bind _outhits (`KismetSystemLibrary.SphereTraceMultiForObjects` _returnvalue (+ _returnvalue (* (`self.GetActorForwardVector`) 50.0)) 100.0 (`|MakeArray` "ObjectTypeQuery3" :!type "EObjectTypeQuery Enum")))
  (`|ExecutionSequence`
    (:`then_0`
      (goto _label :!via `Reset`))
    (:`then_1`
      (for _array_element _outhits
        (`/Engine/EditorBlueprintResources/StandardMacros.DoOnce` false :!label _label
          (:`Completed`
            (bind _asbp_spark_character_player (cast `/Game/Gameplay/Characters/Player/BP_SparkCharacter_Player` (`.HitActor` (`GameplayStatics.BreakHitResult` _array_element))))
            (`GameplayStatics.ApplyDamage` _asbp_spark_character_player 1.0 (`self.GetController`) self "/Game/Gameplay/Logic/DamageTypes/DT_Piercing.DT_Piercing_C")))))))

(event `GruntShieldBash`
  (bind _returnvalue (`SceneComponent.GetSocketLocation` (`self.Mesh`) "LeftHandSocket"))
  ;[1 1 1] Shield bash
  (bind _outhits (`KismetSystemLibrary.SphereTraceMultiForObjects` _returnvalue (+ _returnvalue (* (`self.GetActorForwardVector`) 50.0)) 100.0 (`|MakeArray` "ObjectTypeQuery3" :!type "EObjectTypeQuery Enum")))
  (`|ExecutionSequence`
    (:`then_0`
      (goto _label_2 :!via `Reset`))
    (:`then_1`
      (for _array_element _outhits
        (bind _asbp_spark_character_player (cast `/Game/Gameplay/Characters/Player/BP_SparkCharacter_Player` (`.HitActor` (`GameplayStatics.BreakHitResult` _array_element))))
        (`/Engine/EditorBlueprintResources/StandardMacros.DoOnce` false :!label _label_2
          (:`Completed`
            (`/Game/Gameplay/Characters/Player/BP_SparkCharacter_Player.StopCharging` _asbp_spark_character_player)
            (`self.LaunchCharacter` _asbp_spark_character_player (`KismetMathLibrary.MakeVector` (.x (* (`self.GetActorForwardVector`) 600.0)) (.y (* (`self.GetActorForwardVector`) 600.0)) 300.0) true true)
            (`GameplayStatics.ApplyDamage` _asbp_spark_character_player 1.0 (`self.GetController`) self "/Game/Gameplay/Logic/DamageTypes/DT_Piercing.DT_Piercing_C")))))))

(fn `UserConstructionScript`
  (`parent.UserConstructionScript`)
  ;[1 1 1] Attach the grunt's weapons
  (`SceneComponent.K2_AttachToComponent` (`self.GruntAxeMesh`) (`self.Mesh`) "RightHandSocket" "SnapToTarget" "KeepRelative" "SnapToTarget" true)
  (`SceneComponent.K2_AttachToComponent` (`self.GruntShieldMesh`) (`self.Mesh`) "LeftHandSocket" "SnapToTarget" "KeepRelative" "SnapToTarget" true)
  ;[1 1 1] Make the shield a little bit bigger
  (`SceneComponent.SetRelativeScale3D` (`self.GruntShieldMesh`) (`KismetMathLibrary.Conv_DoubleToVector` 1.25)))