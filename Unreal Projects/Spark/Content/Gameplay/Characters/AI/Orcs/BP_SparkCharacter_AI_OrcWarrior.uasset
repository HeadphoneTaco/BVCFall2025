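; Orc warrior AI character that carries a sword mesh snapped to its right-hand socket in the construction script.
; The WarriorSlash event runs a multi-sphere trace for pawns from that socket along the actor's forward vector.
; A DoOnce, reset each slash, passes only the first hit, which takes piercing damage if it is the player character.
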(event `WarriorSlash`
  (bind _returnvalue (`SceneComponent.GetSocketLocation` (`self.Mesh`) "RightHandSocket"))
  ;[1 1 1] Two handed strong attack
  (bind _outhits (`KismetSystemLibrary.SphereTraceMultiForObjects` _returnvalue (+ _returnvalue (* (`self.GetActorForwardVector`) 120.0)) 100.0 (`|MakeArray` "ObjectTypeQuery3" :!type "EObjectTypeQuery Enum")))
  (`|ExecutionSequence`
    (:`then_0`
      (goto _label :!via `Reset`))
    (:`then_1`
      (for _array_element _outhits
        (`/Engine/EditorBlueprintResources/StandardMacros.DoOnce` false :!label _label
          (:`Completed`
            (bind _asbp_spark_character_player (cast `/Game/Gameplay/Characters/Player/BP_SparkCharacter_Player` (`.HitActor` (`GameplayStatics.BreakHitResult` _array_element))))
            (`GameplayStatics.ApplyDamage` _asbp_spark_character_player 2.0 (`self.GetController`) self "/Game/Gameplay/Logic/DamageTypes/DT_Piercing.DT_Piercing_C")))))))

(fn `UserConstructionScript`
  (`parent.UserConstructionScript`)
  (`SceneComponent.K2_AttachToComponent` (`self.WarriorSwordMesh`) (`self.Mesh`) "RightHandSocket" "SnapToTarget" "KeepRelative" "SnapToTarget" true))