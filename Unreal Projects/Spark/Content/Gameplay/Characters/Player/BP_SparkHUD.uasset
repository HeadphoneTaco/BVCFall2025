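; BP_SparkHUD is the player HUD that manages the mouse cursor, pause menu, guidebook and dialog boxes.
; On BeginPlay it sets a custom cursor widget, and toggling the pause menu or guidebook plays a sound and pushes or pops its widget.
; A widget stack handles viewport add and remove, calling pushed and popped notifications.
; New dialogs join the stack, but RemoveDialogWidget only detaches from the parent, leaving the stack entry.
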(event `self.ReceiveBeginPlay`
  ;[1 1 1] Begin play
  (`self.CreateCursorWidget`))

(event `CreateCursorWidget`
  ;[1 1 1] Cursor widget
  (bind _returnvalue (`|CreateWidget` "/Game/UI/Widgets/Menus/WBP_Cursor.WBP_Cursor_C"))
  (`PlayerController.SetMouseCursorWidget` (`GameplayStatics.GetPlayerController` 0) "Default" _returnvalue))

(fn `CreateDialogWidget`
  (params (BodyText :type Text :default "NSLOCTEXT(\"[0BA0AC2A4B6812C0EA88B38EBA524262]\", \"DB38F3D244883BD0897013BCD39D414E\", \"Body text here.\")") (ConfirmButtonText :type Text :default "NSLOCTEXT(\"[0BA0AC2A4B6812C0EA88B38EBA524262]\", \"FD25029245C283E20BAC8DACADD38B0F\", \"Confirm\")") (CancelButtonText :type Text :default "NSLOCTEXT(\"[0BA0AC2A4B6812C0EA88B38EBA524262]\", \"8AA8BE504997D0A3AA60E98100412C36\", \"Cancel\")"))
  (returns (DialogWidget :type "/Game/UI/Widgets/Menus/WBP_DialogBox Object Reference"))
  (locals (LocalDialogueBox :type "/Game/UI/Widgets/Menus/WBP_DialogBox Object Reference"))
  (bind _returnvalue (`|CreateWidget` "/Game/UI/Widgets/Menus/WBP_DialogBox.WBP_DialogBox_C" (`GameplayStatics.GetPlayerController` 0) BodyText ConfirmButtonText CancelButtonText))
  (set `local.LocalDialogueBox` _returnvalue)
  (`self.Push Widget` (`local.LocalDialogueBox`))
  (return (`local.LocalDialogueBox`)))

(fn `PopWidget`
  (returns (WidgetPopped :type Boolean) (PoppedWidget :type "UserWidget Object Reference") (StackLastIndex :type Integer))
  (locals (LocalStackLastIndex :type Integer :default 0) (LocalPoppedWidget :type "UserWidget Object Reference"))
  (bind _output_get (set `local.LocalStackLastIndex` (`KismetArrayLibrary.Array_LastIndex` (`self.WidgetStack`))))
  (if (>= _output_get 0)
    (bind _output_get_2 (set `local.LocalPoppedWidget` (`|GetArrayItem` (`self.WidgetStack`) (`local.LocalStackLastIndex`))))
    (`Widget.RemoveFromParent` _output_get_2)
    (`KismetArrayLibrary.Array_Remove` (`self.WidgetStack`) (`local.LocalStackLastIndex`))
    (`self.OnWidgetStackPopped` (`local.LocalPoppedWidget`) (`local.LocalStackLastIndex`))
    (return true (`local.LocalPoppedWidget`) (`local.LocalStackLastIndex`))
    (else
      (return false null -1))))

(fn `Push Widget`
  (params (NewWidget :type "UserWidget Object Reference"))
  (returns (PushedIndex :type Integer))
  (locals (LocalWidget :type "UserWidget Object Reference") (LocalPushedIndex :type Integer :default 0))
  (bind _output_get (set `local.LocalWidget` NewWidget))
  (`UserWidget.AddToViewport` _output_get 0)
  (bind _returnvalue (`KismetArrayLibrary.Array_Add` (`self.WidgetStack`) (`local.LocalWidget`)))
  (set `local.LocalPushedIndex` _returnvalue)
  (`self.OnWidgetStackPushed` (`local.LocalWidget`) (`local.LocalPushedIndex`))
  (return (`local.LocalPushedIndex`)))

(fn `RemoveDialogWidget`
  (params (DialogWidget :type "UserWidget Object Reference"))
  (`Widget.RemoveFromParent` DialogWidget))

(fn `SetEnableGuidebook`
  (params (Condition :type Boolean))
  (if Condition
    (`GameplayStatics.PlaySound2D` "/Game/Sound/SFX/Cues/SC_PauseIn.SC_PauseIn" 1.0 1.0 0.0 null null)
    (`self.Push Widget` (`self.GuidebookWidget`))
    (else
      (`GameplayStatics.PlaySound2D` "/Game/Sound/SFX/Cues/SC_PauseOut.SC_PauseOut" 1.0 1.0 0.0 null null)
      (`self.PopWidget`))))

(fn `SetEnablePause Menu`
  (params (Enabled :type Boolean))
  (returns (PauseMenuWidget :type "/Game/UI/Widgets/Menus/WBP_PauseMenu Object Reference"))
  (if Enabled
    (`GameplayStatics.PlaySound2D` "/Game/Sound/SFX/Cues/SC_PauseIn.SC_PauseIn" 1.0 1.0 0.0 null null)
    (`self.Push Widget` (`self.PauseMenuWidget`))
    (else
      (`GameplayStatics.PlaySound2D` "/Game/Sound/SFX/Cues/SC_PauseOut.SC_PauseOut" 1.0 1.0 0.0 null null)
      (`self.PopWidget`)))
  (return (`self.PauseMenuWidget`)))

(fn `UserConstructionScript`)