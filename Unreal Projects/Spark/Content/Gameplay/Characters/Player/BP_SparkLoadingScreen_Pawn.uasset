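; Player pawn for Spark on the loading screen, with fire breath and barrel roll actions.
; Movement axes are only stored in variables here; nothing in this graph moves the pawn.
; Flame plays a montage with a sound and a Niagara effect spawned at the mouth socket, while Jump plays a dodge montage as the roll.
; A shared macro blocks both actions while any montage is playing.
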(event `InputAxis|MoveForward`
  (params (AxisValue :type "Float (single-precision)"))
  ;[1 1 1] Movement
  (set `self.MoveForward` AxisValue))

(event `InputAxis|MoveRight`
  (params (AxisValue :type "Float (single-precision)"))
  ;[1 1 1] Movement
  (set `self.MoveRight` AxisValue))

(event `InputAction|Flame`
  (params (Key :type "Key Structure"))
  ;[1 1 1] Fire breath
  (:`Pressed`
    (`self.IsAnyMontagePlaying`
      (:`false`
        (`AnimInstance.Montage_Play` (`SkeletalMeshComponent.GetAnimInstance` (`self.SkeletalMesh`)) "/Game/Characters/Spark/Animations/A_Spark_FireBreath_Montage.A_Spark_FireBreath_Montage" 1.0 "MontageLength" 0.0 true)
        (`NiagaraFunctionLibrary.SpawnSystemAttached` "/Game/Characters/Spark/FX/FX_FireBreath_System.FX_FireBreath_System" (`self.SkeletalMesh`) "None" (`SceneComponent.GetSocketLocation` (`self.SkeletalMesh`) "MouthSocket") (`self.K2_GetActorRotation`) "KeepWorldPosition" true)
        (`GameplayStatics.PlaySoundAtLocation` "/Game/Characters/Spark/Audio/SC_Flame.SC_Flame" (`self.K2_GetActorLocation`) (struct) 1.0 1.0 0.0 null null null)))))

(event `InputAction|Jump`
  (params (Key :type "Key Structure"))
  ;[1 1 1] Do a barrel roll!
  (:`Pressed`
    (`self.IsAnyMontagePlaying`
      (:`false`
        (`AnimInstance.Montage_Play` (`SkeletalMeshComponent.GetAnimInstance` (`self.SkeletalMesh`)) "/Game/Characters/Spark/Animations/A_Spark_Fly_Dodge_Left_Montage.A_Spark_Fly_Dodge_Left_Montage" 1.0 "MontageLength" 0.0 true)))))

(fn `UserConstructionScript`)