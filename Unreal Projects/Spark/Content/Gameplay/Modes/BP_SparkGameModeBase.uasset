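; Base game mode that sets up game audio and handles level music and loading of the campaign's root level.
; On BeginPlay it activates the global sound mix and applies the saved profile's Master, Effects, Music and Dialog volumes as clamped sound class overrides.
; It also exposes events to swap and play music through MusicManager and to open the root level with game-only input and a hidden cursor.
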(event `self.ReceiveBeginPlay`
  ;[1 1 1] Begin play
  (`self.InitAudioMix`))

(event `InitAudioMix`
  (bind _userprofilesavegame (`/Game/Gameplay/Modes/BP_SparkGameInstance.UserProfileSaveGame` (`/Game/Gameplay/Modes/BPFL_SparkGameModes.GetSparkGameInstance`)))
  ;[1 1 1] Set the base mix for the game
  (`GameplayStatics.SetBaseSoundMix` "/Game/Sound/Mixes/Mix_Global.Mix_Global")
  (`GameplayStatics.PushSoundMixModifier` "/Game/Sound/Mixes/Mix_Global.Mix_Global")
  ;[1 1 1] Set volume levels of various classes
  (`self.SetVolumeSoundClass` "NewEnumerator1" (`/Game/Gameplay/SaveGame/BP_Spark_UserSave.VolumeMaster` _userprofilesavegame))
  (`self.SetVolumeSoundClass` "NewEnumerator2" (`/Game/Gameplay/SaveGame/BP_Spark_UserSave.VolumeSFX` _userprofilesavegame))
  (`self.SetVolumeSoundClass` "NewEnumerator3" (`/Game/Gameplay/SaveGame/BP_Spark_UserSave.VolumeMusic` _userprofilesavegame))
  (`self.SetVolumeSoundClass` "NewEnumerator4" (`/Game/Gameplay/SaveGame/BP_Spark_UserSave.VolumeDialog` _userprofilesavegame)))

(event `SetLevelMusic`
  (params (NewSound :type "SoundBase Object Reference"))
  ;[1 1 1] Set the music volume
  (`/Engine/EditorBlueprintResources/StandardMacros.IsValid` NewSound
    (:`Is Valid`
      (`AudioComponent.SetSound` (`self.MusicManager`) NewSound)
      (`AudioComponent.Play` (`self.MusicManager`) 0.0))))

(event `LoadCampaignGame`
  (bind _returnvalue (`GameplayStatics.GetPlayerController` 0))
  ;[1 1 1] Load the main game level's root level
  (set `PlayerController.bShowMouseCursor` false _returnvalue)
  (`WidgetBlueprintLibrary.SetInputMode_GameOnly` _returnvalue)
  (`GameplayStatics.OpenLevel` (`self.RootLevelFileName`)))

(fn `SetVolumeSoundClass`
  (params (SoundClass :type "/Game/Sound/Classes/ESparkSoundClasses Enum" :default "NewEnumerator0") (Volume :type "Float (double-precision)"))
  (`GameplayStatics.SetSoundMixClassOverride` "/Game/Sound/Mixes/Mix_Global.Mix_Global" (select `/Game/Sound/Classes/ESparkSoundClasses` SoundClass :`NewEnumerator1` "/Game/Sound/Classes/Spark_Master.Spark_Master" :`NewEnumerator2` "/Game/Sound/Classes/Spark_Effects.Spark_Effects" :`NewEnumerator3` "/Game/Sound/Classes/Spark_Music.Spark_Music" :`NewEnumerator4` "/Game/Sound/Classes/Spark_Voice.Spark_Voice" :!type "SoundClass Object Reference") (`KismetMathLibrary.FClamp` Volume) 1.0 0.0)
  (return))

(fn `UserConstructionScript`)