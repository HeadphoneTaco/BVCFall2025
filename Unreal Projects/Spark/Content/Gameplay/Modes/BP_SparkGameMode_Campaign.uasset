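; Campaign game mode that handles player respawning and streamed transitions between hubs and levels.
; On death it fades out and destroys the character, whose destroyed event respawns it at the checkpoint and rebinds.
; Transitions share one white-fade sequence through a randomly timed loading sublevel, spawning at the matching BP_LevelPortal in hubs or "Start" in levels.
; BeginPlay handles initial hub loading or an editor fallback; SpawnDefaultPawnFor offsets pawn height for capsule mismatch.
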(event `self.ReceiveBeginPlay`
  ;[1 1 1] Begin play
  (`parent.ReceiveBeginPlay`)
  (`self.BindPlayerToRespawn`)
  (`self.InitialHubLoad`))

(event `BindPlayerToRespawn`
  ;[1 1 1] Respawn player script
  (bind _asbp_spark_character_player (cast `/Game/Gameplay/Characters/Player/BP_SparkCharacter_Player` (`GameplayStatics.GetPlayerCharacter` 0)))
  (add `/Game/Gameplay/Characters/BP_SparkCharacter.OnCharacterDead` _asbp_spark_character_player (delegate `OnCharacterDead_Event_0`))
  (add `self.OnDestroyed` _asbp_spark_character_player (delegate `OnDestroyed_Event_0`)))

(event `OnCharacterDead_Event_0`
  (params (DeadCharacter :type "/Game/Gameplay/Characters/BP_SparkCharacter Object Reference"))
  ;[1 1 1] Respawn player script
  (`KismetSystemLibrary.Delay` 2.0)
  (`PlayerCameraManager.StartCameraFade` :`self` (`GameplayStatics.GetPlayerCameraManager` 0) :`ToAlpha` 1.0 :`Duration` 0.6 :`bHoldWhenFinished` true)
  (`KismetSystemLibrary.Delay` 0.6)
  (`|ExecutionSequence`
    (:`then_0`
      (`KismetSystemLibrary.Delay` 1.0 :!label _label)
      (`PlayerCameraManager.StartCameraFade` :`self` (`GameplayStatics.GetPlayerCameraManager` 0) :`FromAlpha` 1.0 :`Duration` 1.0 :`bHoldWhenFinished` true)
      (goto _label_2 :!via `Close`))
    (:`then_1`
      (`self.K2_DestroyActor` (`GameplayStatics.GetPlayerCharacter` 0))
      (goto _label_2 :!via `Open`))))

(event `OnDestroyed_Event_0` :!signature `self.OnDestroyed`
  (params (DestroyedActor :type "Actor Object Reference"))
  ;[1 1 1] Respawn player script
  (`self.RestartPlayerAtPlayerStart` (`GameplayStatics.GetPlayerController` 0) (`self.K2_FindPlayerStart` null (`/Game/Gameplay/Modes/BP_SparkGameInstance.GetCheckpointTag` (`/Game/Gameplay/Modes/BPFL_SparkGameModes.GetSparkGameInstance`))))
  (`self.OnPlayerRespawned` (cast `/Game/Gameplay/Characters/Player/BP_SparkCharacter_Player` (`GameplayStatics.GetPlayerCharacter` 0) :!pure true))
  (`self.BindPlayerToRespawn`)
  (`/Engine/EditorBlueprintResources/StandardMacros.Gate` true :!label _label_2
    (:`Exit`
      (goto _label))))

(event `InitialHubLoad`
  (bind _returnvalue (`GameplayStatics.GetPlayerCharacter` 0))
  (bind _rootspawnblockingvolume (`self.RootSpawnBlockingVolume`))
  ;[1 1 1] Initial hub load from main menu
  (if (`/Game/Gameplay/Modes/BP_SparkGameInstance.GetLoadingToRootFromMenu` (`/Game/Gameplay/Modes/BPFL_SparkGameModes.GetSparkGameInstance`))
    (`PlayerCameraManager.StartCameraFade` (`GameplayStatics.GetPlayerCameraManager` 0) 0.0 1.0 0.0 (struct :`R` 1.0 :`G` 1.0 :`B` 1.0 :`A` 1.0) false true)
    (`GameplayStatics.LoadStreamLevel` (`self.LoadingLevelFileName`) true true)
    (`PlayerCameraManager.StartCameraFade` (`GameplayStatics.GetPlayerCameraManager` 0) 1.0 0.0 0.4 (struct :`R` 1.0 :`G` 1.0 :`B` 1.0 :`A` 1.0) false true)
    (`KismetSystemLibrary.Delay` (`KismetMathLibrary.RandomFloatInRange` (`self.MinLevelLoadingTime`) (`self.MaxLevelLoadingTime`)))
    (`PlayerCameraManager.StartCameraFade` (`GameplayStatics.GetPlayerCameraManager` 0) 0.0 1.0 0.4 (struct :`R` 1.0 :`G` 1.0 :`B` 1.0 :`A` 1.0) false true)
    (`KismetSystemLibrary.Delay` 0.5)
    (`/Game/Gameplay/Modes/BP_SparkGameState.SetCurrentSubLevelFileName` (`/Game/Gameplay/Modes/BPFL_SparkGameModes.GetSparkGameState`) (`/Game/Gameplay/Modes/BP_SparkGameInstance.GetCurrentHubFileName` (`/Game/Gameplay/Modes/BPFL_SparkGameModes.GetSparkGameInstance`)))
    (`GameplayStatics.UnloadStreamLevel` (`self.LoadingLevelFileName`) true)
    (`GameplayStatics.LoadStreamLevel` (`/Game/Gameplay/Modes/BP_SparkGameInstance.GetCurrentHubFileName` (`/Game/Gameplay/Modes/BPFL_SparkGameModes.GetSparkGameInstance`)) true)
    (`self.RestartPlayerAtPlayerStart` (`GameplayStatics.GetPlayerController` 0) (`self.K2_FindPlayerStart` null "Start"))
    (`PlayerCameraManager.StartCameraFade` (`GameplayStatics.GetPlayerCameraManager` 0) 1.0 0.0 0.4 (struct :`R` 1.0 :`G` 1.0 :`B` 1.0 :`A` 1.0) false true)
    (`/Engine/EditorBlueprintResources/StandardMacros.IsValid` _rootspawnblockingvolume
      (:`Is Valid`
        (`self.SetActorEnableCollision` _rootspawnblockingvolume false)))
    (else
      ;[1 0 0.08132] This will only get fired while working directly in the editor
      (`/Game/Gameplay/Modes/BP_SparkGameInstance.SetCurrentHubFileName` (`/Game/Gameplay/Modes/BPFL_SparkGameModes.GetSparkGameInstance`) "Level_World_A_HUB")
      (`/Engine/EditorBlueprintResources/StandardMacros.IsValid` _returnvalue
        (:`Is Valid`
          (`self.K2_DestroyActor` _returnvalue))
        (:`Is Not Valid`
          _))
      (`self.RestartPlayerAtPlayerStart` (`GameplayStatics.GetPlayerController` 0) (`self.K2_FindPlayerStart` null (`/Game/Gameplay/Modes/BP_SparkGameInstance.GetCheckpointTag` (`/Game/Gameplay/Modes/BPFL_SparkGameModes.GetSparkGameInstance`)))))))

(event `GetRootSpawnBlockingVolume`
  ;[1 1 1] Get a reference to the root spawn blocking volume under the player start
  (bind _outactors (`GameplayStatics.GetAllActorsWithTag` "RootSpawnBlockingVolume"))
  (set `self.RootSpawnBlockingVolume` (`|GetArrayItem` _outactors)))

(event `TransitionToHUB`
  (params (CurrentLevelFileName :type Name))
  ;[1 1 1] The loading sequence is mostly the same
  (set `self.LevelFileName` CurrentLevelFileName)
  (set `self.LoadingToHub` true)
  ;[1 1 1] Fade to white and disable input
  (`PlayerCameraManager.StartCameraFade` (`GameplayStatics.GetPlayerCameraManager` 0) 0.0 1.0 0.4 (struct :`R` 1.0 :`G` 1.0 :`B` 1.0 :`A` 1.0) false true :!label _label)
  (`self.DisableInput` (`GameplayStatics.GetPlayerController` 0) null)
  (`KismetSystemLibrary.Delay` 0.8)
  ;[1 1 1] Destroy the player, then unload the previous level and load the loading level
  (`self.K2_DestroyActor` (`GameplayStatics.GetPlayerCharacter` 0))
  (`GameplayStatics.UnloadStreamLevel` (select `bool` (`self.LoadingToHub`) :`false` (`/Game/Gameplay/Modes/BP_SparkGameInstance.GetCurrentHubFileName` (`/Game/Gameplay/Modes/BPFL_SparkGameModes.GetSparkGameInstance`)) :`true` (`self.LevelFileName`)) true)
  (`GameplayStatics.LoadStreamLevel` (`self.LoadingLevelFileName`) true true)
  ;[1 1 1] Fade back in and wait in the loading level
  (`PlayerCameraManager.StartCameraFade` (`GameplayStatics.GetPlayerCameraManager` 0) 1.0 0.0 0.4 (struct :`R` 1.0 :`G` 1.0 :`B` 1.0 :`A` 1.0) false true)
  (`KismetSystemLibrary.Delay` (`KismetMathLibrary.RandomFloatInRange` (`self.MinLevelLoadingTime`) (`self.MaxLevelLoadingTime`)))
  ;[1 1 1] Fade out, unload the loading level, then load the destination level
  (`PlayerCameraManager.StartCameraFade` (`GameplayStatics.GetPlayerCameraManager` 0) 0.0 1.0 0.4 (struct :`R` 1.0 :`G` 1.0 :`B` 1.0 :`A` 1.0) false true)
  (`KismetSystemLibrary.Delay` 0.5)
  (`/Game/Gameplay/Modes/BP_SparkGameState.SetCurrentSubLevelFileName` (`/Game/Gameplay/Modes/BPFL_SparkGameModes.GetSparkGameState`) (`self.LevelFileName`))
  (`GameplayStatics.UnloadStreamLevel` (`self.LoadingLevelFileName`) true)
  (`GameplayStatics.LoadStreamLevel` (select `bool` (`self.LoadingToHub`) :`false` (`self.LevelFileName`) :`true` (`/Game/Gameplay/Modes/BP_SparkGameInstance.GetCurrentHubFileName` (`/Game/Gameplay/Modes/BPFL_SparkGameModes.GetSparkGameInstance`))) true)
  (if (`self.LoadingToHub`)
    ;[1 1 1] If we're loading to a hub, find the correct level portal and respawn there
    (bind _outactors (`GameplayStatics.GetAllActorsOfClass` "/Game/Gameplay/Objects/BP_LevelPortal.BP_LevelPortal_C"))
    (for _array_element _outactors
      (if (== (`/Game/Gameplay/Objects/BP_LevelPortal.LevelDestinationFileName` _array_element) (`self.LevelFileName`))
        (set `self.DestinationLevelPortal` _array_element)))
    (`self.RestartPlayerAtTransform` (`GameplayStatics.GetPlayerController` 0) (`SceneComponent.K2_GetComponentToWorld` (`/Game/Gameplay/Objects/BP_LevelPortal.ReturnTeleportLocation` (`self.DestinationLevelPortal`))))
    (else
      ;[1 1 1] If we're going to a world, then load at the player start with the '0' tag
      (`self.RestartPlayerAtPlayerStart` (`GameplayStatics.GetPlayerController` 0) (`self.K2_FindPlayerStart` null "Start"))))
  ;[1 1 1] Restore input and fade up
  (`self.EnableInput` (`GameplayStatics.GetPlayerController` 0) null)
  (`PlayerCameraManager.StartCameraFade` (`GameplayStatics.GetPlayerCameraManager` 0) 1.0 0.0 0.4 (struct :`R` 1.0 :`G` 1.0 :`B` 1.0 :`A` 1.0) false true))

(event `TransitionToLevel`
  (params (DestinationLevelFileName :type Name))
  ;[1 1 1] The loading sequence is mostly the same
  (set `self.LevelFileName` DestinationLevelFileName)
  (set `self.LoadingToHub` false)
  (goto _label))

(fn `ChoosePlayerStart`
  (params (Player :type "Controller Object Reference"))
  (returns (ReturnValue :type "Actor Object Reference"))
  (bind _returnvalue (`parent.ChoosePlayerStart` Player))
  (return _returnvalue))

(fn `SpawnDefaultPawnFor`
  (params (NewPlayer :type "Controller Object Reference") (StartSpot :type "Actor Object Reference"))
  (returns (ReturnValue :type "Pawn Object Reference"))
  (bind _returnvalue (`parent.SpawnDefaultPawnFor` NewPlayer StartSpot))
  ;[1 0 0] This is a terrible hack. The character's capsule height is smaller than the player spawn, so he spawns in the air slightly. There is no easy way to change a player start's capsule height without extending the player start class so here we are.
  (bind _asbp_spark_character_player (cast `/Game/Gameplay/Characters/Player/BP_SparkCharacter_Player` _returnvalue)
    (:`then`
      (`self.K2_AddActorWorldOffset` _asbp_spark_character_player (`KismetMathLibrary.MakeVector` 0.0 0.0 (/ (- (`CapsuleComponent.GetScaledCapsuleHalfHeight` (`Character.CapsuleComponent` _asbp_spark_character_player)) 88.0) 2.0)) false false))
    (:`CastFailed`
      _))
  (return _returnvalue))

(fn `UserConstructionScript`)