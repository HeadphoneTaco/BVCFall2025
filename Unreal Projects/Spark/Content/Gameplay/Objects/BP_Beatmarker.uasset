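; BP_Beatmarker is an in-world text marker that labels a beat and turns to face the player.
; The construction script formats its event, character, object, misc and notes fields into one line on BeatText.
; Every tick, TurnToPlayer smoothly interpolates the Base component's world rotation toward the first player character, using only look-at yaw with a half-turn offset so it stays upright.
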(event `self.ReceiveTick`
  (params (DeltaSeconds :type "Float (single-precision)"))
  (`self.TurnToPlayer`))

(event `TurnToPlayer`
  (bind _returnvalue (`GameplayStatics.GetPlayerCharacter` 0))
  (bind _base (`self.Base`))
  ;[1 1 1] Comment
  (`/Engine/EditorBlueprintResources/StandardMacros.IsValid` _returnvalue
    (:`Is Valid`
      (`SceneComponent.K2_SetWorldRotation` _base (`KismetMathLibrary.RInterpTo` (`SceneComponent.K2_GetComponentRotation` _base) (`KismetMathLibrary.ComposeRotators` (`KismetMathLibrary.MakeRotator` 0.0 0.0 (.yaw (`KismetMathLibrary.FindLookAtRotation` (`self.K2_GetActorLocation` _returnvalue) (`self.K2_GetActorLocation`)))) (struct :`Yaw` 180.0)) (`GameplayStatics.GetWorldDeltaSeconds`) 5.0) false false))))

(fn `UserConstructionScript`
  (`TextRenderComponent.K2_SetText` (`self.BeatText`) (`|FormatText` "- {Event} - \n{Character} \n{Object} \n{Misc} \n- {Notes} -" (`self.Event`) (`self.Character`) (`self.Objects`) (`self.Misc`) (`self.Additional Notes`))))