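; BP_DragonEgg is a collectible egg that hatches a dragon once, when the player overlaps it or it takes any damage.
; Hatching increments the game state's egg count, then plays animations, sounds and colour-tinted stream and burst effects before destroying the actor.
; A construction-script GUID identifies each egg, so BeginPlay destroys those the game instance records as collected.
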(event `self.SphereCollision.OnComponentBeginOverlap`
  (params (OverlappedComponent :type "PrimitiveComponent Object Reference") (OtherActor :type "Actor Object Reference") (OtherComp :type "PrimitiveComponent Object Reference") (OtherBodyIndex :type Integer) (bFromSweep :type Boolean) (SweepResult :type "HitResult Structure (by ref)"))
  (cast `/Game/Gameplay/Characters/Player/BP_SparkCharacter_Player` OtherActor)
  (`/Engine/EditorBlueprintResources/StandardMacros.DoOnce` false :!label _label
    (:`Completed`
      (`PrimitiveComponent.SetCollisionEnabled` (`self.EggMesh`) "NoCollision")
      (`SkeletalMeshComponent.PlayAnimation` (`self.EggMesh`) "/Game/Characters/Egg/Animations/A_Egg_Hatch.A_Egg_Hatch" false)
      (`GameplayStatics.PlaySoundAtLocation` "/Game/Characters/Egg/Sound/SC_Egg_Hatch.SC_Egg_Hatch" (`self.K2_GetActorLocation`) (struct) 1.0 1.0 0.0 null null null)
      (`SkeletalMeshComponent.PlayAnimation` (`self.DragonMesh`) "/Game/Characters/Spark/Animations/A_Spark_Level_Up.A_Spark_Level_Up" false)
      (`AudioComponent.FadeIn` (`self.S_EggSpawning_Loop_Cue`) 0.2 1.0 0.0 "Linear")
      (`/Game/Gameplay/Modes/BP_SparkGameState.IncrementCurrentEggCount` (`/Game/Gameplay/Modes/BPFL_SparkGameModes.GetSparkGameState`) (`self.EggGUID`))
      (`ActorComponent.Activate` (`self.DragonStreamFX`) false)
      (`NiagaraComponent.SetVariableLinearColor` (`self.DragonStreamFX`) "DragonColour" (`self.Color`))
      (`NiagaraComponent.SetVariableLinearColor` (`self.DragonBurstFX`) "DragonColour" (`self.Color`))
      (`KismetSystemLibrary.Delay` 2.4)
      (`ActorComponent.Deactivate` (`self.DragonStreamFX`))
      (`ActorComponent.Activate` (`self.DragonBurstFX`) false)
      (`SceneComponent.SetVisibility` (`self.DragonMesh`) false false)
      (`SceneComponent.K2_DetachFromComponent` (`self.DragonBurstFX`) "KeepWorld" "KeepWorld" "KeepWorld" true)
      (`SceneComponent.K2_DetachFromComponent` (`self.DragonStreamFX`) "KeepWorld" "KeepWorld" "KeepWorld" true)
      (`GameplayStatics.PlaySoundAtLocation` "/Game/Characters/Egg/Sound/S_EggSpawning_Burst_Cue.S_EggSpawning_Burst_Cue" (`self.K2_GetActorLocation`) (struct) 1.0 1.0 0.0 null null null)
      (`AudioComponent.FadeOut` (`self.S_EggSpawning_Loop_Cue`) 1.0 0.0 "Linear")
      (`KismetSystemLibrary.Delay` 5.0)
      (`self.K2_DestroyActor`))))

(event `self.ReceiveBeginPlay`
  ;[1 1 1] Comment
  (if (`/Game/Gameplay/Modes/BP_SparkGameInstance.IsItemCollected` (`/Game/Gameplay/Modes/BPFL_SparkGameModes.GetSparkGameInstance`) "NewEnumerator2" (`self.EggGUID`))
    (`self.K2_DestroyActor`)))

(event `self.ReceiveAnyDamage`
  (params (Damage :type "Float (single-precision)") (DamageType :type "DamageType Object Reference") (InstigatedBy :type "Controller Object Reference") (DamageCauser :type "Actor Object Reference"))
  (goto _label))

(fn `UserConstructionScript`
  ;[1 1 1] Generate a unique GUID for the egg
  (if (not (`KismetGuidLibrary.IsValid_Guid` (`self.EggGUID`)))
    (set `self.EggGUID` (`KismetGuidLibrary.NewGuid`))))