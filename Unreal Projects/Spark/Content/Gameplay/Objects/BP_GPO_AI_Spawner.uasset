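; Gameplay object that spawns a Spark AI character from its archetype class, either automatically at BeginPlay or through SpawnAI.
; SpawnAI places the pawn slightly above the spawner, copies Gems onto it, caches the character and AI controller, and broadcasts OnCharacterSpawned.
; Auto-spawned characters also have their death relayed through the spawner's OnCharacterDead for easy scripting.
; GetSparkAI returns the cached references.
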(event `self.ReceiveBeginPlay`
  ;[1 1 1] Check if auto spawn is set to true
  (if (`self.AutoSpawn`)
    (bind _spark_ai_character (`self.SpawnAI`))
    ;[1 1 1] Pass this thru for easy scripting
    (add `/Game/Gameplay/Characters/BP_SparkCharacter.OnCharacterDead` _spark_ai_character (delegate `OnCharacterDead_Event_0`))))

(event `OnCharacterDead_Event_0`
  (params (DeadCharacter :type "/Game/Gameplay/Characters/BP_SparkCharacter Object Reference"))
  ;[1 1 1] Pass this thru for easy scripting
  (`self.OnCharacterDead` DeadCharacter))

(fn `GetSparkAI`
  (returns (SparkAICharacter :type "/Game/Gameplay/Characters/AI/BP_SparkCharacter_AI Object Reference") (SparkAIController :type "/Game/Gameplay/Characters/AI/BP_SparkAIController Object Reference"))
  (return (`self.SparkAICharacter`) (`self.SparkAIController`)))

(fn `SpawnAI`
  (returns (`Spark AI Character` :type "/Game/Gameplay/Characters/AI/BP_SparkCharacter_AI Object Reference") (`Spark AI Controller` :type "/Game/Gameplay/Characters/AI/BP_SparkAIController Object Reference"))
  (bind _returnvalue (`AIBlueprintHelperLibrary.SpawnAIFromClass` (`self.AIArchetype`) null (+ (.location (`self.GetTransform`)) (0.0 0.0 44.0)) (.rotation (`self.GetTransform`)) true null))
  (bind _asbp_spark_character_ai (cast `/Game/Gameplay/Characters/AI/BP_SparkCharacter_AI` _returnvalue :!pure true))
  (set `/Game/Gameplay/Characters/AI/BP_SparkCharacter_AI.Gems` (`self.Gems`) _asbp_spark_character_ai)
  (set `self.SparkAICharacter` _asbp_spark_character_ai)
  (set `self.SparkAIController` (cast `/Game/Gameplay/Characters/AI/BP_SparkAIController` (`AIBlueprintHelperLibrary.GetAIController` _asbp_spark_character_ai) :!pure true))
  (`self.OnCharacterSpawned` (`self.SparkAICharacter`) (`self.SparkAIController`))
  (return (`self.SparkAICharacter`) (`self.SparkAIController`)))

(fn `UserConstructionScript`)