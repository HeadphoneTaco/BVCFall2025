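; Geyser gameplay object that pushes the Spark player upward while inside its capsule, unless the player is gliding.
; It runs constantly or alternates on active/inactive timers, toggling sound, Niagara, post process and a timeline-scaled water spout.
; Tick applies the force through two gates, one for eruption state and one for player overlap.
; The construction script derives capsule size, spout scale and particle velocity from VentHeight.
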(event `self.ReceiveTick`
  (params (DeltaSeconds :type "Float (single-precision)"))
  (`/Engine/EditorBlueprintResources/StandardMacros.Gate` true :!label _label
    (:`Exit`
      ;[1 1 1] Only apply the force if the player is inside the geyser volume
      (`/Engine/EditorBlueprintResources/StandardMacros.Gate` true :!label _label_2
        (:`Exit`
          (`self.ApplyUpwardForce` (stale `self.GeyserCollision.OnComponentBeginOverlap` _asbp_spark_character_player)))))))

(event `StartGeyser`
  ;[1 1 1] Kick off the FX
  (`GameplayStatics.PlaySoundAtLocation` "/Game/Objects/Geyser/Sound/SC_Geyser_Erupt.SC_Geyser_Erupt" (`self.K2_GetActorLocation`) (struct) 1.0 1.0 0.0 null null null)
  (`AudioComponent.FadeIn` (`self.GeyserLoopSFX`) 1.0 1.0 0.0 "Linear")
  (`ActorComponent.Activate` (`self.GeyserVFX`) true)
  (`ActorComponent.Activate` (`self.Niagara`) true)
  (set `PostProcessComponent.bEnabled` true (`self.PostProcess1`))
  (`self.PlayGeyserAnimation`)
  (goto _label :!via `Open`))

(event `Activate`
  ;[1 1 1] Whether or not to always be active or not
  (if (not (`self.GeyserAlwaysActive`)) :!label _label_3
    (`self.StartActiveTimer`))
  (`self.StartGeyser`))

(event `self.ReceiveBeginPlay`
  ;[1 1 1] Whether or not to always be active or not
  (if (`self.GeyserStartActive`)
    (goto _label_3)
    (else
      (`self.StopGeyser`))))

(event `StopGeyser`
  ;[1 1 1] Kick off the FX
  (`AudioComponent.FadeOut` (`self.GeyserLoopSFX`) 1.0 0.0 "Linear")
  (`ActorComponent.Deactivate` (`self.GeyserVFX`))
  (`ActorComponent.Deactivate` (`self.Niagara`))
  (set `PostProcessComponent.bEnabled` false (`self.PostProcess1`))
  (`self.ReverseGeyserAnimation`)
  (goto _label :!via `Close`))

(event `StartActiveTimer`
  ;[1 1 1] Cooldowns
  (`KismetSystemLibrary.Delay` (`self.GeyserActiveTime`))
  (`self.StopGeyser`)
  (`self.StartInactiveTimer`))

(event `self.GeyserCollision.OnComponentBeginOverlap`
  (params (OverlappedComponent :type "PrimitiveComponent Object Reference") (OtherActor :type "Actor Object Reference") (OtherComp :type "PrimitiveComponent Object Reference") (OtherBodyIndex :type Integer) (bFromSweep :type Boolean) (SweepResult :type "HitResult Structure (by ref)"))
  ;[1 1 1] Only apply the force if the player is inside the geyser volume
  (bind _asbp_spark_character_player (cast `/Game/Gameplay/Characters/Player/BP_SparkCharacter_Player` OtherActor))
  (goto _label_2 :!via `Open`))

(event `StartInactiveTimer`
  ;[1 1 1] Cooldowns
  (`KismetSystemLibrary.Delay` (`self.GeyserInactiveTime`))
  (`self.StartGeyser`)
  (`self.StartActiveTimer`))

(event `self.GeyserCollision.OnComponentEndOverlap`
  (params (OverlappedComponent :type "PrimitiveComponent Object Reference") (OtherActor :type "Actor Object Reference") (OtherComp :type "PrimitiveComponent Object Reference") (OtherBodyIndex :type Integer))
  ;[1 1 1] Only apply the force if the player is inside the geyser volume
  (cast `/Game/Gameplay/Characters/Player/BP_SparkCharacter_Player` OtherActor)
  (goto _label_2 :!via `Close`))

(event `PlayGeyserAnimation`
  ;[1 1 1] Geyser Animation
  (`SceneComponent.SetVisibility` (`self.SM_WaterSpoutv2`) true false)
  (`SceneComponent.SetVisibility` (`self.Cylinder`) true false)
  (bind (_direction _alpha) (`Timeline|GeyserRisingTimeline` :!label _label_4)
    (:`Update`
      (`SceneComponent.SetWorldScale3D` (`self.WaterBaseScaleScene`) (`KismetMathLibrary.MakeVector` 1.0 1.0 (`KismetMathLibrary.Lerp` 0.0 (/ (`self.VentHeight`) 100.0) _alpha))))
    (:`Finished`
      (switch `ETimelineDirection` _direction
        (:`Backward`
          (`SceneComponent.SetVisibility` (`self.SM_WaterSpoutv2`) false false)
          (`SceneComponent.SetVisibility` (`self.Cylinder`) false false))))))

(event `ReverseGeyserAnimation`
  ;[1 1 1] Geyser Animation
  (goto _label_4 :!via `Reverse`))

(fn `ApplyUpwardForce`
  (params (PlayerCharacter :type "/Game/Gameplay/Characters/Player/BP_SparkCharacter_Player Object Reference"))
  (`/Engine/EditorBlueprintResources/StandardMacros.IsValid` PlayerCharacter
    (:`Is Valid`
      (if (not (`/Game/Gameplay/Characters/Player/BP_SparkCharacter_Player.GetIsGliding` PlayerCharacter))
        (`CharacterMovementComponent.AddForce` (`Character.CharacterMovement` PlayerCharacter) (`self.UpwardForce`))))))

(fn `SetForceCapsuleHeight`
  (bind _returnvalue (+ (/ (`self.VentHeight`) 2.0) (/ (`CapsuleComponent.CapsuleRadius` (`self.GeyserCollision`)) 2.0)))
  (`CapsuleComponent.SetCapsuleHalfHeight` (`self.GeyserCollision`) _returnvalue true)
  (`SceneComponent.K2_SetRelativeLocation` (`self.GeyserCollision`) (`KismetMathLibrary.MakeVector` 0.0 0.0 (- _returnvalue (`CapsuleComponent.CapsuleRadius` (`self.GeyserCollision`)))) false false))

(fn `UserConstructionScript`
  (bind _returnvalue (`KismetSystemLibrary.MakeLiteralDouble` (* (`self.VentHeight`) 2.0)))
  (`self.SetForceCapsuleHeight`)
  (`TimelineComponent.SetPlayRate` (`self.GeyserRisingTimeline`) (/ 1.0 (`self.GeyserRiseSpeed`)))
  (`SceneComponent.SetWorldScale3D` (`self.WaterBaseScaleScene`) (`KismetMathLibrary.MakeVector` 1.0 1.0 (/ (`self.VentHeight`) 100.0)))
  (`SceneComponent.K2_AttachToComponent` (`self.SM_WaterSpoutv2`) (`self.Cylinder`) "WaterTubeTop" "SnapToTarget" "KeepWorld" "KeepWorld" true)
  (`SceneComponent.K2_AddWorldOffset` (`self.SM_WaterSpoutv2`) (`KismetMathLibrary.MakeVector` 0.0 0.0 -20.0) false false)
  (`FXSystemComponent.SetFloatParameter` (`self.GeyserVFX`) "VelocityMin" _returnvalue)
  (`FXSystemComponent.SetFloatParameter` (`self.GeyserVFX`) "VelocityMax" _returnvalue))