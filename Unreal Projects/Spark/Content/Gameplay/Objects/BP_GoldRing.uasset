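; BP_GoldRing is a one-shot collectible ring that the player spark character picks up by overlapping it.
; Overlap with its cylinder casts to the player character and passes a DoOnce gate, so the pickup fires only once.
; It then plays the pickup sound, stops the Niagara effect, spawns a coloured BP_Gem at its transform, hides the mesh and destroys itself after a short delay.
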(event `self.Cylinder.OnComponentBeginOverlap`
  (params (OverlappedComponent :type "PrimitiveComponent Object Reference") (OtherActor :type "Actor Object Reference") (OtherComp :type "PrimitiveComponent Object Reference") (OtherBodyIndex :type Integer) (bFromSweep :type Boolean) (SweepResult :type "HitResult Structure (by ref)"))
  (cast `/Game/Gameplay/Characters/Player/BP_SparkCharacter_Player` OtherActor)
  (`/Engine/EditorBlueprintResources/StandardMacros.DoOnce` false
    (:`Completed`
      (`GameplayStatics.PlaySoundAtLocation` "/Game/Objects/Ring/Sound/SC_Ring_Pickup.SC_Ring_Pickup" (`self.K2_GetActorLocation`) (struct) 1.0 1.0 0.0 null null null)
      (`ActorComponent.Deactivate` (`self.Niagara`))
      (`|SpawnActorFromClass` "/Game/Gameplay/Objects/BP_Gem.BP_Gem_C" (`self.GetTransform`) "Undefined" "OverrideRootScale" null "NewEnumerator4" (struct) null)
      (`SceneComponent.SetVisibility` (`self.StaticMesh`) false false)
      (`KismetSystemLibrary.Delay` 3.0)
      (`self.K2_DestroyActor`))))

(fn `UserConstructionScript`)