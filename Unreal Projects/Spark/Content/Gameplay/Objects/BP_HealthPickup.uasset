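; BP_HealthPickup is a meat health pickup that heals the player on overlap, only when they are below max health.
; Healing is applied as negative damage through ApplyDamage, using the flame breath damage type.
; On pickup it plays an eating sound and Niagara effect at the player's mouth socket, then destroys itself.
; A FloatingMeat timeline, slowed at BeginPlay, defines the mesh's vertical bob, though no Play call is wired.
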(event `self.ReceiveBeginPlay`
  ;[1 1 1] Set the timing on floating animation
  (`TimelineComponent.SetPlayRate` (`self.FloatingMeat`) (/ 1.0 2.0)))

(event `self.HealthCollision.OnComponentBeginOverlap`
  (params (OverlappedComponent :type "PrimitiveComponent Object Reference") (OtherActor :type "Actor Object Reference") (OtherComp :type "PrimitiveComponent Object Reference") (OtherBodyIndex :type Integer) (bFromSweep :type Boolean) (SweepResult :type "HitResult Structure (by ref)"))
  ;[1 1 1] Only pick it up if the player is missing health
  (bind _asbp_spark_character_player (cast `/Game/Gameplay/Characters/Player/BP_SparkCharacter_Player` OtherActor))
  (if (not (`/Game/Gameplay/Characters/BP_SparkCharacter.IsAtMaxHealth` _asbp_spark_character_player))
    ;[1 1 1] Heal
    (`GameplayStatics.ApplyDamage` _asbp_spark_character_player (* (`self.HealValue`) -1.0) null null "/Game/Gameplay/Logic/DamageTypes/DT_FlameBreath.DT_FlameBreath_C")
    (bind _location (.location (`SceneComponent.GetSocketTransform` (`Character.Mesh` _asbp_spark_character_player) "MouthSocket" "RTS_World")))
    (bind _rotation (.rotation (`SceneComponent.GetSocketTransform` (`Character.Mesh` _asbp_spark_character_player) "MouthSocket" "RTS_World")))
    ;[1 1 1] Play FX then destroy
    (`GameplayStatics.PlaySoundAtLocation` "/Game/Objects/HealthPickup/Sound/S_HealthPickup_Eat_Cue.S_HealthPickup_Eat_Cue" _location (struct) 1.0 1.0 0.0 null null null)
    (`NiagaraFunctionLibrary.SpawnSystemAtLocation` "/Game/Objects/HealthPickup/FX/FX_HealthPickup_System.FX_HealthPickup_System" (+ _location (* (`KismetMathLibrary.GetForwardVector` _rotation) 10.0)) _rotation)
    (`self.K2_DestroyActor`)))

(fn `UserConstructionScript`)