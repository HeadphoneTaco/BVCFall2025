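; BP_LevelPortal is a placeable portal that sends the player to another level.
; On begin play it writes the destination's display and designer names into two 3D WBP_LevelPortal widgets.
; The construction script disables widget shadows and applies a dynamic material instance showing the destination cubemap on both portal planes.
; When a BP_SparkCharacter_Player overlaps PortalCollision, a DoOnce-gated call asks the Spark campaign game mode to transition to the destination level.
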(event `SetPortalWidgetText`
  ;[1 1 1] Set the text on the widgets
  (for _array_element (`|MakeArray` (`self.Widget`) (`self.Widget1`))
    (bind _aswbp_level_portal (cast `/Game/UI/Widgets/InGame/WBP_LevelPortal` (`WidgetComponent.GetUserWidgetObject` _array_element) :!pure true))
    (`/Game/UI/Widgets/InGame/WBP_LevelPortal.SetWorldNameText` _aswbp_level_portal (`self.LevelDestinationDisplayName`))
    (`/Game/UI/Widgets/InGame/WBP_LevelPortal.SetDesignerNameText` _aswbp_level_portal (`self.LevelDestinationDesignerName`))))

(event `self.ReceiveBeginPlay`
  ;[1 1 1] Begin play
  (`self.SetPortalWidgetText`))

(event `self.PortalCollision.OnComponentBeginOverlap`
  (params (OverlappedComponent :type "PrimitiveComponent Object Reference") (OtherActor :type "Actor Object Reference") (OtherComp :type "PrimitiveComponent Object Reference") (OtherBodyIndex :type Integer) (bFromSweep :type Boolean) (SweepResult :type "HitResult Structure (by ref)"))
  ;[1 1 1] Transition to the level
  (cast `/Game/Gameplay/Characters/Player/BP_SparkCharacter_Player` OtherActor)
  (`/Engine/EditorBlueprintResources/StandardMacros.DoOnce` false
    (:`Completed`
      (`/Game/Gameplay/Modes/BP_SparkGameMode_Campaign.TransitionToLevel` (`/Game/Gameplay/Modes/BPFL_SparkGameModes.GetSparkGameModeCampaign`) (`self.LevelDestinationFileName`)))))

(fn `UserConstructionScript`
  ;[1 1 1] Remove the shadows from the 3D widgets
  (`PrimitiveComponent.SetCastShadow` (`self.Widget1`) false)
  (`PrimitiveComponent.SetCastShadow` (`self.Widget`) false)
  ;[1 1 1] Create the DMI for the portal
  (bind _returnvalue (`KismetMaterialLibrary.CreateDynamicMaterialInstance` "/Game/Objects/LevelPortal/Materials/M_LevelPortal_Inst.M_LevelPortal_Inst"))
  (`MaterialInstanceDynamic.SetTextureParameterValue` _returnvalue "Cubemap" (`self.LevelTextureCube`))
  (`PrimitiveComponent.SetMaterial` (`self.PortalPlane02`) 0 _returnvalue)
  (`PrimitiveComponent.SetMaterial` (`self.PortalPlane01`) 0 _returnvalue))