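; A floating cloud platform that vanishes a set delay after the player lands on it, then respawns.
; Its collision is off by default and turns on only while the player overlaps the volume above it and the platform is solid.
; The first player hit starts a recursive one-second countdown through a DoOnce gate.
; At zero, audio and particles stop before collision is disabled, and a respawn delay later restores them and resets the gate.
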(event `self.ReceiveBeginPlay`
  (`PrimitiveComponent.SetCollisionEnabled` (`self.PlatformCollision`) "NoCollision"))

(event `DecrementTime`
  (`/Engine/EditorBlueprintResources/StandardMacros.CompareFloat` (`self.CurrentTimeToGo`)
    (:`>`
      (set `self.CurrentTimeToGo` (- (`self.CurrentTimeToGo`) 1.0))
      (`KismetSystemLibrary.Delay` 1.0)
      (`self.DecrementTime`))
    (:`==`
      (set `self.CurrentTimeToGo` 0.0)
      (`AudioComponent.FadeOut` (`self.Audio`) 1.0 0.0 "Linear")
      (`ActorComponent.Deactivate` (`self.CloudParticles`))
      (`KismetSystemLibrary.Delay` 1.5)
      (set `self.IsSolid` false)
      (`PrimitiveComponent.SetCollisionEnabled` (`self.PlatformCollision`) "NoCollision")
      (`KismetSystemLibrary.Delay` (`self.RespawnTime`))
      (`self.RespawnPlatform`))))

(event `self.PlatformCollision.OnComponentHit`
  (params (HitComponent :type "PrimitiveComponent Object Reference") (OtherActor :type "Actor Object Reference") (OtherComp :type "PrimitiveComponent Object Reference") (NormalImpulse :type "Vector Structure") (Hit :type "HitResult Structure (by ref)"))
  (cast `/Game/Gameplay/Characters/Player/BP_SparkCharacter_Player` OtherActor)
  (`/Engine/EditorBlueprintResources/StandardMacros.DoOnce` false :!label _label
    (:`Completed`
      (set `self.CurrentTimeToGo` (`self.DelayDisappearTime`))
      (`self.DecrementTime`))))

(event `RespawnPlatform`
  (`AudioComponent.FadeIn` (`self.Audio`) 1.0 1.0 0.0 "Linear")
  (`NiagaraComponent.ResetSystem` (`self.CloudParticles`))
  (set `self.IsSolid` true)
  (goto _label :!via `Reset`))

(event `self.AbovePlatformCollision.OnComponentBeginOverlap`
  (params (OverlappedComponent :type "PrimitiveComponent Object Reference") (OtherActor :type "Actor Object Reference") (OtherComp :type "PrimitiveComponent Object Reference") (OtherBodyIndex :type Integer) (bFromSweep :type Boolean) (SweepResult :type "HitResult Structure (by ref)"))
  (cast `/Game/Gameplay/Characters/Player/BP_SparkCharacter_Player` OtherActor)
  (if (`self.IsSolid`)
    (`PrimitiveComponent.SetCollisionEnabled` (`self.PlatformCollision`) "QueryAndPhysics")))

(event `self.AbovePlatformCollision.OnComponentEndOverlap`
  (params (OverlappedComponent :type "PrimitiveComponent Object Reference") (OtherActor :type "Actor Object Reference") (OtherComp :type "PrimitiveComponent Object Reference") (OtherBodyIndex :type Integer))
  (cast `/Game/Gameplay/Characters/Player/BP_SparkCharacter_Player` OtherActor)
  (if (`self.IsSolid`)
    (`PrimitiveComponent.SetCollisionEnabled` (`self.PlatformCollision`) "NoCollision")))

(fn `UserConstructionScript`)