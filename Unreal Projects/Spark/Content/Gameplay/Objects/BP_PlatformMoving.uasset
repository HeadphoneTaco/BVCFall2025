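; Moving platform that travels between its start transform and a relative end offset, optionally auto-playing after an initial delay.
; A timeline interpolates the cube's location and rotation, with its play rate derived from TimeToMove in the construction script.
; A looping sound fades in and out with movement.
; On arrival it fires OnPlatformFinishedMoving, pauses, then ping-pongs if Looping; MovePlatform and ReversePlatform allow external control.
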(event `StartLoopingAudio`
  (`AudioComponent.FadeIn` (`self.SC_MovingPlatform_Loop`) 0.5 1.0 0.0 "Linear"))

(event `self.ReceiveBeginPlay`
  (bind (_starttransform_location _starttransform_rotation _starttransform_scale) (`KismetMathLibrary.BreakTransform` (`self.StartTransform`)))
  (bind (_endtransform_location _endtransform_rotation) (`KismetMathLibrary.BreakTransform` (`self.EndTransform`)))
  (bind (_starttransform_location_2 _starttransform_rotation_2) (`KismetMathLibrary.BreakTransform` (`self.StartTransform`)))
  ;[1 1 1] Save the initial transform
  (set `self.StartTransform` (`SceneComponent.K2_GetComponentToWorld` (`self.Cube`)))
  ;[1 1 1] Are we set to auto play
  (if (`self.AutoPlay`)
    ;[1 1 1] Initial delay
    (`KismetSystemLibrary.Delay` (`self.InitialDelay`))
    (`self.StartLoopingAudio` :!label _label)
    ;[1 1 1] Moving platform
    (bind (_direction _alpha) (`Timeline|MovingPlatform` :!label _label_2)
      (:`Update`
        (`SceneComponent.K2_SetWorldTransform` (`self.Cube`) (`KismetMathLibrary.MakeTransform` (`KismetMathLibrary.VLerp` _starttransform_location_2 (+ _starttransform_location_2 _endtransform_location) _alpha) (`KismetMathLibrary.RLerp` _starttransform_rotation_2 (`KismetMathLibrary.ComposeRotators` _starttransform_rotation_2 _endtransform_rotation) _alpha true) _starttransform_scale) false false))
      (:`Finished`
        (`AudioComponent.FadeOut` (`self.SC_MovingPlatform_Loop`) 0.5 0.0 "Linear")
        ;[1 1 1] Looping behaviour
        (`self.OnPlatformFinishedMoving` _direction)
        (`KismetSystemLibrary.Delay` (`self.StoppedDelay`))
        (if (`self.Looping`)
          (switch `ETimelineDirection` _direction
            (:`Forward`
              (`self.ReversePlatform`))
            (:`Backward`
              (`self.MovePlatform`))))))))

(event `MovePlatform`
  ;[1 1 1] For external use
  (goto _label))

(event `ReversePlatform`
  ;[1 1 1] For external use
  (`self.StartLoopingAudio`)
  (goto _label_2 :!via `Reverse`))

(fn `UserConstructionScript`
  ;[1 1 1] Comment
  (`TimelineComponent.SetPlayRate` (`self.MovingPlatform`) (/ 1.0 (`self.TimeToMove`))))