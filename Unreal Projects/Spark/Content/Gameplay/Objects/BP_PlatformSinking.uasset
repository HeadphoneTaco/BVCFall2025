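; Sinking platform that drops along Z when the player lands on it, then rises after a delay, with splash and bubble sounds.
; An overlap volume flags the player as on top, gating the mesh hit that plays the sinking timeline.
; A second timeline eases each move in by ramping the sinking timeline's play rate.
; A wobble timeline, with no wired trigger, holds mesh tilt logic scaled by player presence.
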(event `self.ReceiveBeginPlay`
  ;[1 1 1] Store the location of the mesh
  (set `self.StartLocation` (`SceneComponent.K2_GetComponentLocation` (`self.SinkingPlatformMesh`))))

(event `self.SinkingPlatformMesh.OnComponentHit`
  (params (HitComponent :type "PrimitiveComponent Object Reference") (OtherActor :type "Actor Object Reference") (OtherComp :type "PrimitiveComponent Object Reference") (NormalImpulse :type "Vector Structure") (Hit :type "HitResult Structure (by ref)"))
  (bind _returnvalue (`self.K2_GetActorLocation`))
  (bind _startlocation (`self.StartLocation`))
  ;[1 1 1] When the player jumps onto the platform
  (bind _asbp_spark_character_player (cast `/Game/Gameplay/Characters/Player/BP_SparkCharacter_Player` OtherActor))
  (if (`self.IsPlayerOnTopOfPlatform`)
    (`/Engine/EditorBlueprintResources/StandardMacros.IsValid` _asbp_spark_character_player
      (:`Is Valid`
        (add `Character.MovementModeChangedDelegate` _asbp_spark_character_player (delegate `MovementModeChangedDelegate_Event_0`))
        ;[1 1 1] Sink up and down animation
        (`self.EaseInMovement`)
        (bind (_direction _alpha) (`Timeline|SinkingTimeline` :!label _label)
          (:`Update`
            (`SceneComponent.K2_SetWorldLocation` (`self.SinkingPlatformMesh`) (`KismetMathLibrary.VLerp` _startlocation (+ _startlocation (`self.EndLocation`)) _alpha) false false))
          (:`Finished`
            (switch `ETimelineDirection` _direction
              (:`Forward`
                (`KismetSystemLibrary.Delay` (`self.SinkStopDelay`))
                (`self.EaseInMovement`)
                (goto _label :!via `Reverse`))))
          (:`SplashSFX`
            ;[1 1 1] Comment
            (`GameplayStatics.PlaySoundAtLocation` "/Game/Objects/SinkingPlatform/Sound/SC_SinkingPlatform_Splash.SC_SinkingPlatform_Splash" _returnvalue (struct) 1.0 1.0 0.0 null null null))
          (:`BubblesSFX`
            (`GameplayStatics.PlaySoundAtLocation` "/Game/Objects/SinkingPlatform/Sound/SC_SinkingPlatform_Bubbles.SC_SinkingPlatform_Bubbles" _returnvalue (struct) 1.0 1.0 0.0 null null null)))))))

(event `self.SinkingPlatformCollision.OnComponentBeginOverlap`
  (params (OverlappedComponent :type "PrimitiveComponent Object Reference") (OtherActor :type "Actor Object Reference") (OtherComp :type "PrimitiveComponent Object Reference") (OtherBodyIndex :type Integer) (bFromSweep :type Boolean) (SweepResult :type "HitResult Structure (by ref)"))
  ;[1 1 1] Detect when the player is on top of the platform
  (cast `/Game/Gameplay/Characters/Player/BP_SparkCharacter_Player` OtherActor)
  (set `self.IsPlayerOnTopOfPlatform` true)
  (set `self.WobbleScaleFactor` 5.0))

(event `self.SinkingPlatformCollision.OnComponentEndOverlap`
  (params (OverlappedComponent :type "PrimitiveComponent Object Reference") (OtherActor :type "Actor Object Reference") (OtherComp :type "PrimitiveComponent Object Reference") (OtherBodyIndex :type Integer))
  ;[1 1 1] Detect when the player is on top of the platform
  (cast `/Game/Gameplay/Characters/Player/BP_SparkCharacter_Player` OtherActor)
  (set `self.IsPlayerOnTopOfPlatform` false)
  (set `self.WobbleScaleFactor` 2.0))

(event `MovementModeChangedDelegate_Event_0`
  (params (Character :type "Character Object Reference") (PrevMovementMode :type "EMovementMode Enum" :default "MOVE_None") (PreviousCustomMode :type Byte))
  ;[1 1 1] Player has left the platform
  (if (or (`|EnumEquality` PrevMovementMode "MOVE_Walking") (`|EnumEquality` PrevMovementMode "MOVE_Swimming"))
    (`/Engine/EditorBlueprintResources/StandardMacros.IsValid` (stale `self.SinkingPlatformMesh.OnComponentHit` _asbp_spark_character_player)
      (:`Is Valid`
        (remove `Character.MovementModeChangedDelegate` (stale `self.SinkingPlatformMesh.OnComponentHit` _asbp_spark_character_player) (delegate `MovementModeChangedDelegate_Event_0`))))))

(event `EaseInMovement`
  ;[1 1 1] I couldn't think of a better way to do this - could probably use cubic interp instead of another timeline - oh well
  (bind (_direction _alpha) (`Timeline|EaseInEaseOutTimeline` :!via `PlayFromStart` :!label _label_2)
    (:`Update`
      (`TimelineComponent.SetPlayRate` (`self.SinkingTimeline`) (* _alpha (/ 1.0 (`self.TimeToSink`)))))))

(event `EaseOutMovement`
  ;[1 1 1] I couldn't think of a better way to do this - could probably use cubic interp instead of another timeline - oh well
  (goto _label_2 :!via `ReverseFromEnd`))

(fn `UserConstructionScript`
  (bind (_endlocation_x _endlocation_y _endlocation_z) (`KismetMathLibrary.BreakVector` (`self.EndLocation`)))
  ;[1 1 1] Comment
  (`TimelineComponent.SetPlayRate` (`self.SinkingTimeline`) (/ 1.0 (`self.TimeToSink`)))
  ;[1 1 1] Comment
  (set `self.EndLocation` (`KismetMathLibrary.MakeVector` 0.0 0.0 _endlocation_z))
  ;[1 1 1] Comment
  (`TimelineComponent.SetPlayRate` (`self.WobblyTimeline`) (`KismetMathLibrary.RandomFloatInRange` 0.08 0.12))
  ;[1 1 1] Comment
  (`TimelineComponent.SetPlayRate` (`self.EaseInEaseOutTimeline`) (/ 1.0 (`self.SinkStopDelay`))))