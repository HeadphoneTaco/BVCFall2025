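; BP_ReturnPortal is a level portal that lets the player leave and return to the hub.
; Overlapping EnterCollision pauses the game, switches to UI input and opens a confirmation dialog; confirming transitions to the hub, while either choice restores game controls.
; A DoOnce blocks repeat prompts until any end overlap on the separate ExitCollision resets it.
; Each tick, its widget smoothly yaws toward the player.
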(event `self.ReceiveTick`
  (params (DeltaSeconds :type "Float (single-precision)"))
  ;[1 1 1] Tick
  (`self.TurnWidgetToPlayer`))

(event `TurnWidgetToPlayer`
  (bind _returnvalue (`GameplayStatics.GetPlayerCharacter` 0))
  (bind _widget (`self.Widget`))
  ;[1 1 1] Rotate the widget to the player
  (`/Engine/EditorBlueprintResources/StandardMacros.IsValid` _returnvalue
    (:`Is Valid`
      (`SceneComponent.K2_SetWorldRotation` _widget (`KismetMathLibrary.RInterpTo` (`SceneComponent.K2_GetComponentRotation` _widget) (`KismetMathLibrary.ComposeRotators` (`KismetMathLibrary.MakeRotator` 0.0 0.0 (.yaw (`KismetMathLibrary.FindLookAtRotation` (`self.K2_GetActorLocation` _returnvalue) (`self.K2_GetActorLocation`)))) (struct :`Yaw` 180.0)) (`GameplayStatics.GetWorldDeltaSeconds`) 5.0) false false))))

(event `self.EnterCollision.OnComponentBeginOverlap`
  (params (OverlappedComponent :type "PrimitiveComponent Object Reference") (OtherActor :type "Actor Object Reference") (OtherComp :type "PrimitiveComponent Object Reference") (OtherBodyIndex :type Integer) (bFromSweep :type Boolean) (SweepResult :type "HitResult Structure (by ref)"))
  ;[1 1 1] When the player enters
  (cast `/Game/Gameplay/Characters/Player/BP_SparkCharacter_Player` OtherActor)
  (`/Engine/EditorBlueprintResources/StandardMacros.DoOnce` false :!label _label
    (:`Completed`
      ;[1 1 1] Pause the game and set controls to the UI mode
      (`GameplayStatics.SetGamePaused` true)
      (set `PlayerController.bShowMouseCursor` true (`GameplayStatics.GetPlayerController` 0))
      (`WidgetBlueprintLibrary.SetInputMode_UIOnlyEx` (`GameplayStatics.GetPlayerController` 0) null)
      ;[1 1 1] Create a dialogue box asking them if they really want to return
      (bind _dialogwidget (`/Game/Gameplay/Characters/Player/BP_SparkHUD.CreateDialogWidget` (`/Game/Gameplay/Modes/BPFL_SparkGameModes.GetSparkHUD`) "Are you sure you want to exit the level and return to the hub?" "Return to the hub" "Stay in the level"))
      (add `/Game/UI/Widgets/Menus/WBP_DialogBox.OnConfirmed` _dialogwidget (delegate `OnConfirmed_Event_0`))
      (add `/Game/UI/Widgets/Menus/WBP_DialogBox.OnCancelled` _dialogwidget (delegate `OnCancelled_Event_0`)))))

(event `self.ExitCollision.OnComponentEndOverlap`
  (params (OverlappedComponent :type "PrimitiveComponent Object Reference") (OtherActor :type "Actor Object Reference") (OtherComp :type "PrimitiveComponent Object Reference") (OtherBodyIndex :type Integer))
  ;[1 1 1] When the player enters
  (goto _label :!via `Reset`))

(event `OnConfirmed_Event_0`
  ;[1 1 1] They accepted, load back
  (`self.SetControlModeToGame`)
  (`/Game/Gameplay/Modes/BP_SparkGameMode_Campaign.TransitionToHUB` (`/Game/Gameplay/Modes/BPFL_SparkGameModes.GetSparkGameModeCampaign`) (`self.LevelFileName`)))

(event `OnCancelled_Event_0`
  ;[1 1 1] They cancelled, return controls
  (`self.SetControlModeToGame`))

(event `SetControlModeToGame`
  ;[1 1 1] Give them back controls
  (`GameplayStatics.SetGamePaused` false)
  (set `PlayerController.bShowMouseCursor` false (`GameplayStatics.GetPlayerController` 0))
  (`WidgetBlueprintLibrary.SetInputMode_GameOnly` (`GameplayStatics.GetPlayerController` 0)))

(fn `UserConstructionScript`)