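; BP_SpeedStrip is a directional boost strip that grants turbo charge to the player's Spark character.
; On overlap with its collision component, a dot product checks that the player is behind or level with the strip relative to its forward vector.
; If that player is already charging, the strip enables turbo charge and plays a boost sound at the player's location.
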(event `self.SpeedStripCollision.OnComponentBeginOverlap`
  (params (OverlappedComponent :type "PrimitiveComponent Object Reference") (OtherActor :type "Actor Object Reference") (OtherComp :type "PrimitiveComponent Object Reference") (OtherBodyIndex :type Integer) (bFromSweep :type Boolean) (SweepResult :type "HitResult Structure (by ref)"))
  (bind _asbp_spark_character_player (cast `/Game/Gameplay/Characters/Player/BP_SparkCharacter_Player` OtherActor))
  (bind _returnvalue (`self.K2_GetActorLocation` _asbp_spark_character_player))
  (if (<= (`KismetMathLibrary.Dot_VectorVector` (`self.GetActorForwardVector`) (`KismetMathLibrary.GetForwardVector` (`KismetMathLibrary.FindLookAtRotation` (`self.K2_GetActorLocation`) _returnvalue))) 0.0)
    (if (`/Game/Gameplay/Characters/Player/BP_SparkCharacter_Player.GetIsCharging` _asbp_spark_character_player)
      (`/Game/Gameplay/Characters/Player/BP_SparkCharacter_Player.EnableTurboCharge` _asbp_spark_character_player)
      (`GameplayStatics.PlaySoundAtLocation` "/Game/Objects/SpeedStrip/Sound/S_Boost_Cue.S_Boost_Cue" _returnvalue (struct) 1.0 1.0 0.0 null null null))))

(fn `UserConstructionScript`)