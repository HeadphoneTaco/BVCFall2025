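; Timed ground spike trap that rises from the floor and deals piercing damage to overlapping actors.
; Construction script tiles instanced spike and base meshes across SpikeSize and fits the damage box to it using mesh bounds.
; A timeline, rate-scaled by Speed, lifts the spikes by mesh height, with event tracks toggling damage collision and sounds.
; It can auto-start after a delay or be triggered externally, optionally looping.
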(event `self.BoxDamageCollision.OnComponentBeginOverlap`
  (params (OverlappedComponent :type "PrimitiveComponent Object Reference") (OtherActor :type "Actor Object Reference") (OtherComp :type "PrimitiveComponent Object Reference") (OtherBodyIndex :type Integer) (bFromSweep :type Boolean) (SweepResult :type "HitResult Structure (by ref)"))
  ;[1 1 1] Damage!
  (`GameplayStatics.ApplyDamage` OtherActor (`self.DamageAmount`) null self "/Game/Gameplay/Logic/DamageTypes/DT_Piercing.DT_Piercing_C"))

(event `TriggerGroundSpikes`
  (params (Looping :type Boolean))
  (bind _returnvalue (`self.K2_GetActorLocation`))
  (bind _startlocation (`self.StartLocation`))
  ;[1 1 1] Event for external calling and looping
  (set `self.Looping` Looping)
  ;[1 1 1] Begin SFX
  (`GameplayStatics.PlaySoundAtLocation` "/Game/Objects/GroundSpikes/Sound/SC_GroundSpike_Begin.SC_GroundSpike_Begin" (`self.K2_GetActorLocation`) (struct) 1.0 1.0 0.0 null null null)
  ;[1 1 1] Animation
  (bind (_direction _alpha) (`Timeline|SpikeAnimationTimeline` :!via `PlayFromStart`)
    (:`Update`
      (`SceneComponent.K2_SetWorldLocation` (`self.GroundSpikeInstancedStaticMesh`) (`KismetMathLibrary.VLerp` _startlocation (+ _startlocation (`KismetMathLibrary.MakeVector` 0.0 0.0 (`self.MeshHeight`))) _alpha) false false))
    (:`Finished`
      ;[1 1 1] Retrigger the ground spikes if we're looping
      (`KismetSystemLibrary.Delay` (`self.LoopingDelay`))
      (if (`self.Looping`)
        (`self.TriggerGroundSpikes` (`self.Looping`))))
    (:`ToggleDamageOn`
      ;[1 1 1] Toggle the collision on and off
      (`PrimitiveComponent.SetCollisionEnabled` (`self.BoxDamageCollision`) "QueryOnly")
      ;[1 1 1] Extend and retract SFX
      (`GameplayStatics.PlaySoundAtLocation` "/Game/Objects/GroundSpikes/Sound/SC_GroundSpike_Extend.SC_GroundSpike_Extend" _returnvalue (struct) 1.0 1.0 0.0 null null null))
    (:`ToggleDamageOff`
      (`PrimitiveComponent.SetCollisionEnabled` (`self.BoxDamageCollision`) "NoCollision")
      (`GameplayStatics.PlaySoundAtLocation` "/Game/Objects/GroundSpikes/Sound/SC_GroundSpike_Retract.SC_GroundSpike_Retract" _returnvalue (struct) 1.0 1.0 0.0 null null null))))

(event `self.ReceiveBeginPlay`
  ;[1 1 1] Store the initial location for animation
  (set `self.StartLocation` (`SceneComponent.K2_GetComponentLocation` (`self.GroundSpikeInstancedStaticMesh`)))
  ;[1 1 1] Check if we should activate
  (if (`self.AutoActivate`)
    ;[1 1 1] Wait for the delay
    (`KismetSystemLibrary.Delay` (+ (`self.InitialDelay`) (/ (`self.Speed`) 1.0)))
    ;[1 1 1] Set the spikes to trigger
    (`self.TriggerGroundSpikes` (`self.Looping`))))

(fn `UserConstructionScript`
  (bind _spikeresized_x (`KismetMathLibrary.BreakVector2D` (`self.SpikeResized`)))
  (bind (_spikeresized_x_2 _spikeresized_y) (`KismetMathLibrary.BreakVector2D` (`self.SpikeResized`)))
  (bind _meshspacing (`self.MeshSpacing`))
  (bind (_spikesize_x _spikesize_y) (`KismetMathLibrary.BreakVector2D` (`self.SpikeSize`)))
  (bind (_spikeresized_x_3 _spikeresized_y_2) (`KismetMathLibrary.BreakVector2D` (`self.SpikeResized`)))
  (bind _spikeresized_x_4 (`KismetMathLibrary.BreakVector2D` (`self.SpikeResized`)))
  (bind _damageboxxyleeway (`self.DamageBoxXYLeeway`))
  (bind (_spikeresized_x_5 _spikeresized_y_3) (`KismetMathLibrary.BreakVector2D` (`self.SpikeResized`)))
  (bind _returnvalue (/ _meshspacing 4.0))
  ;[1 1 1] Dynamically get the height of the mesh
  (set `self.MeshHeight` (.z (`.Max` (`StaticMeshComponent.GetLocalBounds` (`self.GroundSpikeInstancedStaticMesh`)))))
  ;[1 1 1] Comment
  (set `self.MeshSpacing` (* (.x (`.Max` (`StaticMeshComponent.GetLocalBounds` (`self.GroundBaseInstancedStaticMesh`)))) 2.0))
  ;[1 1 1] Recalculate the size of the spikes due to box extents being x2
  (set `self.SpikeResized` (`KismetMathLibrary.MakeVector2D` (`KismetMathLibrary.Conv_IntToDouble` (`KismetMathLibrary.Round` (/ _spikesize_x 2.0))) (`KismetMathLibrary.Conv_IntToDouble` (`KismetMathLibrary.Round` (/ _spikesize_y 2.0)))))
  ;[1 1 1] Set the size of the box extents and add some leeway
  (`BoxComponent.SetBoxExtent` (`self.BoxDamageCollision`) (`KismetMathLibrary.MakeVector` (- _spikeresized_x_5 _damageboxxyleeway) (- _spikeresized_y_3 _damageboxxyleeway) (/ (`self.MeshHeight`) 2.0)) true)
  ;[1 1 1] Set the speed of the spikes animation
  (`TimelineComponent.SetPlayRate` (`self.SpikeAnimationTimeline`) (/ 1.0 (`self.Speed`)))
  ;[1 1 1] Disable collision
  (`PrimitiveComponent.SetCollisionEnabled` (`self.BoxDamageCollision`) "NoCollision")
  ;[1 1 1] Set the correct offset of the spike mesh
  (`SceneComponent.K2_AddLocalOffset` (`self.GroundSpikeInstancedStaticMesh`) (`KismetMathLibrary.MakeVector` 0.0 0.0 (* (+ (`self.MeshHeight`) 3.0) -1.0)) false false)
  ;[1 1 1] Instantiate the instanced meshes
  (for _index (range (+ (`KismetMathLibrary.FTrunc` (* (/ _spikeresized_y (`self.MeshSpacing`)) 2.0)) 1))
    (for _index_2 (range (+ (`KismetMathLibrary.FTrunc` (* (/ _spikeresized_x_4 (`self.MeshSpacing`)) 2.0)) 1))
      (bind _returnvalue_2 (`KismetMathLibrary.MakeVector` (- (+ (* _index_2 (`self.MeshSpacing`)) _returnvalue) _spikeresized_x) (- (+ (* _index _meshspacing) _returnvalue) _spikeresized_y_2)))
      (`InstancedStaticMeshComponent.AddInstance` (`self.GroundSpikeInstancedStaticMesh`) (`KismetMathLibrary.MakeTransform` _returnvalue_2))
      (`InstancedStaticMeshComponent.AddInstance` (`self.GroundBaseInstancedStaticMesh`) (`KismetMathLibrary.MakeTransform` (`KismetMathLibrary.MakeVector` (.x _returnvalue_2) (.y _returnvalue_2) -24.0))))))