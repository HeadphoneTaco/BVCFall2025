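; BP_NotedPro is a level note actor showing header, message, icon and priority color on a camera-facing widget.
; A looping construction-script timer drives updates in editor, and a gate macro switches to Actor Tick during play.
; Each update refreshes the widget, visibility and filtered note list, tethers cable child actors from a spline to target actors, and throttles tick interval by listed note count.
; Construction copies filter and visibility settings to all notes.
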(event `self.ReceiveTick`
  (params (DeltaSeconds :type "Float (single-precision)"))
  (`self.Select Tick Type` :!label _label)
  (`self.Set hidden state tick`)
  (`self.Hidden state tick in game`)
  (`self.Get and set note tool ref`)
  (`self.Make note face Camera`)
  (`self.Set note text`)
  (`self.Set icon image`)
  (`self.Set note priority levels`)
  (`self.Get and make array of all other notes`)
  (`self.Tether system`)
  (`self.Tether scale`)
  (`self.Scroll Padding`)
  (`self.General note optimization`))

(event `Utility Tick`
  (goto _label :!via `Utility Base Tick In`))

(event `self.ReceiveBeginPlay`
  (goto _label :!via `Event Begin Play In`))

(fn `Add Tether / End Point Func`
  (params (Actor :type "Object Object Reference"))
  (returns (`AsTether Cable` :type "/Game/Tools/NotedPro/NotedProFiles/Tethering/BP_NotedPro_TetherCable Object Reference") (`AsTether Cable Endpoint` :type "/Game/Tools/NotedPro/NotedProFiles/Tethering/BP_NotedPro_TetherCableEndpoint Object Reference"))
  (`/Engine/EditorBlueprintResources/StandardMacros.IsValid` Actor
    (:`Is Valid`
      (bind _returnvalue (`AddComponent|NODE_AddChildActorComponent-8`))
      (`ChildActorComponent.SetChildActorClass` _returnvalue "/Game/Tools/NotedPro/NotedProFiles/Tethering/BP_NotedPro_TetherCable.BP_NotedPro_TetherCable_C")
      (bind _asbp_noted_pro_tether_cable (cast `/Game/Tools/NotedPro/NotedProFiles/Tethering/BP_NotedPro_TetherCable` (`ChildActorComponent.ChildActor` _returnvalue)))
      (return _asbp_noted_pro_tether_cable (cast `/Game/Tools/NotedPro/NotedProFiles/Tethering/BP_NotedPro_TetherCableEndpoint` (`ChildActorComponent.ChildActor` (`/Game/Tools/NotedPro/NotedProFiles/Tethering/BP_NotedPro_TetherCable.Tether_Cable_Endpoint (NtoN)` _asbp_noted_pro_tether_cable)) :!pure true)))))

(fn `Add Tether Endpoint Func`
  (returns (`AsTether Cable Endpoint` :type "/Game/Tools/NotedPro/NotedProFiles/Tethering/BP_NotedPro_TetherCableEndpoint Object Reference"))
  (bind _returnvalue (`AddComponent|NODE_AddChildActorComponent-5` :`self` (`self.Current actor ref`)))
  (`ChildActorComponent.SetChildActorClass` _returnvalue "/Game/Tools/NotedPro/NotedProFiles/Tethering/BP_NotedPro_TetherCableEndpoint.BP_NotedPro_TetherCableEndpoint_C")
  (bind _asbp_noted_pro_tether_cable_endpoint (cast `/Game/Tools/NotedPro/NotedProFiles/Tethering/BP_NotedPro_TetherCableEndpoint` (`ChildActorComponent.ChildActor` _returnvalue)))
  (return _asbp_noted_pro_tether_cable_endpoint))

(fn `Cable on spline logic`
  (for _array_element (`self.Tether struct`)
    (bind ((`TetherCableRef_7_0DFF6CD5427D42CEE397EAAB8EF5F38A` _tethercableref) (`ActorRefToPointTo_8_874215DA4771F934062E1A9C277482D5` _actorreftopointto)) (break `/Game/Tools/NotedPro/NotedProFiles/Tethering/SNotedProTether` _array_element))
    (`/Engine/EditorBlueprintResources/StandardMacros.IsValid` _actorreftopointto
      (:`Is Valid`
        (`self.K2_SetActorLocation` _tethercableref (`SplineComponent.FindLocationClosestToWorldLocation` (`self.Spline pointer`) (`self.K2_GetActorLocation` _actorreftopointto) "World") false false)
        (`self.SetActorTickInterval` _tethercableref (`self.Tick Delay`))
        (`self.SetActorTickInterval` _actorreftopointto (`self.Tick Delay`))
        (if (== (`GameplayStatics.GetObjectClass` _actorreftopointto) "BP_NotedPro_C")
          (bind _asbp_noted_pro (cast `/Game/Tools/NotedPro/BP_NotedPro` _actorreftopointto))
          (`self.K2_SetActorLocation` (cast `/Game/Tools/NotedPro/NotedProFiles/Tethering/BP_NotedPro_TetherCableEndpoint` (`ChildActorComponent.ChildActor` (`/Game/Tools/NotedPro/NotedProFiles/Tethering/BP_NotedPro_TetherCable.Tether_Cable_Endpoint (NtoN)` _tethercableref)) :!pure true) (`SplineComponent.FindLocationClosestToWorldLocation` (`/Game/Tools/NotedPro/BP_NotedPro.Spline pointer` _asbp_noted_pro) (`self.K2_GetActorLocation` _tethercableref) "World") false true)))
      (:`Is Not Valid`
        (`self.K2_DestroyActor` _tethercableref)
        (`KismetArrayLibrary.Array_RemoveItem` (`self.Tether struct`) _array_element)))))

(fn `Create attach remove cables`
  (locals (`Note tool ref local` :type "/Game/Tools/NotedPro/NotedProFiles/Widget/WBP_NotedPro Object Reference"))
  ;[1 1 1] If actor is deleted this prevents a cable creation runaway.
  (for _array_element (`self.Tether struct`)
    (`self.K2_DestroyActor` (`.TetherCableRef_7_0DFF6CD5427D42CEE397EAAB8EF5F38A` (break `/Game/Tools/NotedPro/NotedProFiles/Tethering/SNotedProTether` _array_element))))
  (`KismetArrayLibrary.Array_Clear` (`self.Tether struct`))
  ;[1 1 1] Make cable actor and add it to array
  (for _array_element_2 (`self.Point to actors`)
    (bind _output_get (set `self.Current actor ref` _array_element_2))
    ;;[1 1 1] Dont make this into a funtion...Everying blows up when this becomes a function?!
    (`/Engine/EditorBlueprintResources/StandardMacros.IsValid` _output_get
      (:`Is Valid`
        (bind _returnvalue (`AddComponent|NODE_AddChildActorComponent-4`))
        (`ChildActorComponent.SetChildActorClass` _returnvalue "/Game/Tools/NotedPro/NotedProFiles/Tethering/BP_NotedPro_TetherCable.BP_NotedPro_TetherCable_C")
        (bind _asbp_noted_pro_tether_cable (cast `/Game/Tools/NotedPro/NotedProFiles/Tethering/BP_NotedPro_TetherCable` (`ChildActorComponent.ChildActor` _returnvalue)))
        (`KismetArrayLibrary.Array_Add` (`self.Tether struct`) (make `/Game/Tools/NotedPro/NotedProFiles/Tethering/SNotedProTether` _asbp_noted_pro_tether_cable (`self.Current actor ref`) (cast `/Game/Tools/NotedPro/NotedProFiles/Tethering/BP_NotedPro_TetherCableEndpoint` (`ChildActorComponent.ChildActor` (`/Game/Tools/NotedPro/NotedProFiles/Tethering/BP_NotedPro_TetherCable.Tether_Cable_Endpoint (NtoN)` _asbp_noted_pro_tether_cable)) :!pure true))))))
  ;[1 1 1] Set cable attachments
  (for _array_element_3 (`self.Tether struct`)
    (bind _output_get_2 (`self.Get and set note tool ref`))
    (bind ((`TetherCableRef_7_0DFF6CD5427D42CEE397EAAB8EF5F38A` _tethercableref) (`ActorRefToPointTo_8_874215DA4771F934062E1A9C277482D5` _actorreftopointto)) (break `/Game/Tools/NotedPro/NotedProFiles/Tethering/SNotedProTether` _array_element_3))
    (`/Game/Tools/NotedPro/NotedProFiles/Tethering/BP_NotedPro_TetherCable.Attach Cable Func` _tethercableref _actorreftopointto (`Image.ColorAndOpacity` (`/Game/Tools/NotedPro/NotedProFiles/Widget/WBP_NotedPro.NoteBackgroundColor` _output_get_2))))
  ;[1 1 1] Remove unwanted cables
  (for _array_element_4 (`self.Tether struct`)
    (bind ((`TetherCableRef_7_0DFF6CD5427D42CEE397EAAB8EF5F38A` _tethercableref_2) (`ActorRefToPointTo_8_874215DA4771F934062E1A9C277482D5` _actorreftopointto_2)) (break `/Game/Tools/NotedPro/NotedProFiles/Tethering/SNotedProTether` _array_element_4))
    (`/Engine/EditorBlueprintResources/StandardMacros.IsValid` _actorreftopointto_2
      (:`Is Not Valid`
        (`/Engine/EditorBlueprintResources/StandardMacros.IsValid` _tethercableref_2
          (:`Is Valid`
            (`self.K2_DestroyActor` _tethercableref_2))
          (:`Is Not Valid`
            _))
        (`KismetArrayLibrary.Array_RemoveItem` (`self.Tether struct`) _array_element_4)))))

(fn `General note optimization`
  (bind _array_length (`self.Array length`))
  (bind _array_length_2 (`self.Array length`))
  (bind _array_length_3 (`self.Array length`))
  (bind _array_length_4 (`self.Array length`))
  (bind _array_length_5 (`self.Array length`))
  (bind _array_length_6 (`self.Array length`))
  ;[1 1 1] Optimize tick interval based on # of Notes in level
  (set `self.Array length` (`KismetArrayLibrary.Array_Length` (`self.List of other Notes`)))
  (`|ExecutionSequence`
    (:`then_0`
      (`|ExecutionSequence`
        (:`then_0`
          (`self.SetActorTickInterval` (`self.Tick Delay`)))
        (:`then_1`
          (if (and (>= _array_length 0) (< _array_length 10))
            (set `self.Tick Delay` 0.0)))))
    (:`then_1`
      (if (and (>= _array_length_2 10) (< _array_length_2 20))
        (set `self.Tick Delay` 0.03)))
    (:`then_2`
      (if (and (>= _array_length_3 20) (< _array_length_3 30))
        (set `self.Tick Delay` 0.1)))
    (:`then_3`
      (if (and (>= _array_length_4 30) (< _array_length_4 40))
        (set `self.Tick Delay` 0.3)))
    (:`then_4`
      (if (and (>= _array_length_5 40) (< _array_length_5 50))
        (set `self.Tick Delay` 0.4)))
    (:`then_5`
      (if (and (>= _array_length_6 50) (< _array_length_6 75))
        (set `self.Tick Delay` 1.0)))
    (:`then_6`
      (if (>= (`self.Array length`) 75)
        (set `self.Tick Delay` 1.5)))))

(fn `Get and make array of all other notes`
  ;[1 1 1] Setting and clearing all variable arrays
  (`KismetArrayLibrary.Array_Clear` (`self.Notes /Names`))
  (`KismetArrayLibrary.Array_Clear` (`self.Array of all note refs`))
  (`KismetArrayLibrary.Array_Clear` (`self.List of other Notes`))
  (bind _outactors (`GameplayStatics.GetAllActorsOfClass` "BP_NotedPro_C"))
  (bind _output_get (set `self.Array of all note refs` _outactors))
  (for _array_element _output_get
    (set `self.Current note ref` _array_element)
    (if (`|EnumEquality` "NewEnumerator3" (`/Game/Tools/NotedPro/BP_NotedPro.Priority level` (`self.Current note ref`)))
      (`KismetArrayLibrary.Array_Add` (`self.List of other Notes`) (`KismetTextLibrary.Conv_StringToText` (`KismetStringLibrary.Concat_StrStr` (`KismetTextLibrary.Conv_TextToString` (`/Game/Tools/NotedPro/BP_NotedPro.Header / Topic` (`self.Current note ref`))) "- FIXED")))
      (else
        (`KismetArrayLibrary.Array_Add` (`self.List of other Notes`) (`/Game/Tools/NotedPro/BP_NotedPro.Header / Topic` (`self.Current note ref`))))))
  ;;[1 1 1] Set which variables make it through for sorting
  (for (_array_element_2 _array_index) (`self.Array of all note refs`)
    (bind _t_or_f (`self.Sort out notes` _array_element_2))
    (if _t_or_f
      (`KismetArrayLibrary.Array_Add` (`self.Notes /Names`) (make `/Game/Tools/NotedPro/NotedProFiles/Structs/SNotedProInfo` (`|GetArrayItem` (`self.List of other Notes`) _array_index) _array_element_2)))))

(fn `Get and set note tool ref`
  (returns (Output_Get :type "/Game/Tools/NotedPro/NotedProFiles/Widget/WBP_NotedPro Object Reference"))
  (locals (`Note tool ref local` :type "/Game/Tools/NotedPro/NotedProFiles/Widget/WBP_NotedPro Object Reference"))
  (bind _aswbp_noted_pro (cast `/Game/Tools/NotedPro/NotedProFiles/Widget/WBP_NotedPro` (`WidgetComponent.GetUserWidgetObject` (`self.Widget`))))
  (bind _output_get (set `local.Note tool ref local` _aswbp_noted_pro))
  (return _output_get))

(fn `Hidden state tick in game`
  (if (and (`self.Hide in game?`) (`self.Game playing?`))
    (`self.SetActorTickEnabled` false)
    (else
      (return))))

(fn `Make note face Camera`
  (bind (_returnvalue_x _returnvalue_y _returnvalue_z) (`KismetMathLibrary.BreakVector` (`PlayerCameraManager.GetCameraLocation` (`GameplayStatics.GetPlayerCameraManager` 0))))
  (bind (_camera_location_in_editor_x _camera_location_in_editor_y _camera_location_in_editor_z) (`KismetMathLibrary.BreakVector` (`/Game/Tools/NotedPro/NotedProFiles/UtilityBP/BPU_CameraInfo.Camera location in editor` (cast `/Game/Tools/NotedPro/NotedProFiles/UtilityBP/BPU_CameraInfo` (`ChildActorComponent.ChildActor` (`self.Utlity_Camera_Info`)) :!pure true))))
  (`self.Note tilt offset`)
  (if (`self.Game playing?`)
    (`SceneComponent.K2_SetWorldRotation` (`self.Scene`) (`KismetMathLibrary.FindLookAtRotation` (`KismetMathLibrary.MakeVector` _returnvalue_x _returnvalue_y (- _returnvalue_z (`self.Note tilt offset `))) (`self.K2_GetActorLocation`)) false false)
    (else
      (`SceneComponent.K2_SetWorldRotation` (`self.Scene`) (`KismetMathLibrary.FindLookAtRotation` (`KismetMathLibrary.MakeVector` _camera_location_in_editor_x _camera_location_in_editor_y (- _camera_location_in_editor_z (`self.Note tilt offset `))) (`self.K2_GetActorLocation`)) false false))))

(fn `Note tilt offset`
  (set `self.Note tilt offset ` (`KismetMathLibrary.Lerp` 20.0 80.0 (`KismetMathLibrary.MapRangeClamped` (`self.Size of note`) 0.2 2.0 0.0 1.0)))
  (return))

(fn `Pass Global Note Variables to Party`
  (locals (`Local Notes ref` :type "Array of /Game/Tools/NotedPro/BP_NotedPro Object Reference"))
  (bind _outactors (`GameplayStatics.GetAllActorsOfClass` "BP_NotedPro_C"))
  (bind _output_get (set `local.Local Notes ref` _outactors))
  (for _array_element _output_get
    (set `/Game/Tools/NotedPro/BP_NotedPro.Sort by: Icon Statues` (`self.Sort by: Icon Statues`) _array_element)
    (set `/Game/Tools/NotedPro/BP_NotedPro.Sort by: Priority Level` (`self.Sort by: Priority Level`) _array_element)
    (set `/Game/Tools/NotedPro/BP_NotedPro.Sort by: Team members` (`self.Sort by: Team members`) _array_element)
    (`self.Set hidden state tick`)
    (set `/Game/Tools/NotedPro/BP_NotedPro.Note visibility` (`self.Note visibility`) _array_element)))

(fn `Scroll Calculations +`
  (returns (ReturnValue :type "Float (double-precision)"))
  (bind _scrollbox_main (`/Game/Tools/NotedPro/NotedProFiles/Widget/WBP_NotedPro.ScrollBox_main` (cast `/Game/Tools/NotedPro/NotedProFiles/Widget/WBP_NotedPro` (`WidgetComponent.GetUserWidgetObject` (`self.Widget`)) :!pure true)))
  (bind (_returnvalue_x _returnvalue_y) (`KismetMathLibrary.BreakVector2D` (`Widget.GetDesiredSize` _scrollbox_main)))
  (bind (_returnvalue_x_2 _returnvalue_y_2) (`KismetMathLibrary.BreakVector2D` (`SlateBlueprintLibrary.GetLocalSize` (`Widget.GetCachedGeometry` _scrollbox_main))))
  (return (`KismetMathLibrary.FClamp` (+ (`ScrollBox.GetScrollOffset` _scrollbox_main) (`self.Scroll move ammount`)) 0.0 (- _returnvalue_y _returnvalue_y_2))))

(fn `Scroll Calculations -`
  (returns (ReturnValue :type "Float (double-precision)"))
  (bind _scrollbox_main (`/Game/Tools/NotedPro/NotedProFiles/Widget/WBP_NotedPro.ScrollBox_main` (cast `/Game/Tools/NotedPro/NotedProFiles/Widget/WBP_NotedPro` (`WidgetComponent.GetUserWidgetObject` (`self.Widget`)) :!pure true)))
  (bind (_returnvalue_x _returnvalue_y) (`KismetMathLibrary.BreakVector2D` (`Widget.GetDesiredSize` _scrollbox_main)))
  (bind (_returnvalue_x_2 _returnvalue_y_2) (`KismetMathLibrary.BreakVector2D` (`SlateBlueprintLibrary.GetLocalSize` (`Widget.GetCachedGeometry` _scrollbox_main))))
  (return (`KismetMathLibrary.FClamp` (- (`ScrollBox.GetScrollOffset` _scrollbox_main) (`self.Scroll move ammount`)) 0.0 (- _returnvalue_y _returnvalue_y_2))))

(fn `Scroll Padding`
  (bind _scrollbox_main (`/Game/Tools/NotedPro/NotedProFiles/Widget/WBP_NotedPro.ScrollBox_main` (cast `/Game/Tools/NotedPro/NotedProFiles/Widget/WBP_NotedPro` (`WidgetComponent.GetUserWidgetObject` (`self.Widget`)) :!pure true)))
  (bind (_returnvalue_x _returnvalue_y) (`KismetMathLibrary.BreakVector2D` (`Widget.GetDesiredSize` _scrollbox_main)))
  (bind (_returnvalue_x_2 _returnvalue_y_2) (`KismetMathLibrary.BreakVector2D` (`SlateBlueprintLibrary.GetLocalSize` (`Widget.GetCachedGeometry` _scrollbox_main))))
  (bind _asvertical_box_slot (cast `VerticalBoxSlot` (`Widget.Slot` (`/Game/Tools/NotedPro/NotedProFiles/Widget/WBP_NotedPro.NoteText` (cast `/Game/Tools/NotedPro/NotedProFiles/Widget/WBP_NotedPro` (`WidgetComponent.GetUserWidgetObject` (`self.Widget`)) :!pure true))) :!pure true))
  (if (> _returnvalue_y _returnvalue_y_2)
    (`VerticalBoxSlot.SetPadding` _asvertical_box_slot (make `Margin` 0.0 0.0 50.0))
    (else
      (`VerticalBoxSlot.SetPadding` _asvertical_box_slot (make `Margin` 0.0)))))

(fn `Set hidden state tick`
  (bind _scene (`self.Scene`))
  ;[1 1 1] Hidden states are set here
  (switch `/Game/Tools/NotedPro/NotedProFiles/Enums/ENotedProHide` (`self.Note visibility`)
    (:`NewEnumerator0`
      (set `self.Is Hidden in Editor?` false)
      (set `self.Hide in game?` true))
    (:`NewEnumerator1`
      (set `self.Is Hidden in Editor?` false)
      (set `self.Hide in game?` false))
    (:`NewEnumerator2`
      (set `self.Is Hidden in Editor?` true)
      (set `self.Hide in game?` true)))
  (if (`self.Game playing?`)
    (if (`self.Hide in game?`)
      (`SceneComponent.SetVisibility` _scene false true :!label _label)
      (else
        (`SceneComponent.SetVisibility` _scene true true :!label _label_2)))
    (elif (`KismetStringLibrary.Contains` (`KismetSystemLibrary.GetEngineVersion`) "4.22")
      (if (`self.Is Hidden in Editor?`)
        (goto _label)
        (else
          (goto _label_2))))))

(fn `Set icon image`
  (bind (_note _fixit _eye _lighting _sound _player _questionmark _exclamationmark _bp _c__ _generic _geometry _texture _trash _heart _happyface _sadface _neutralface _landscape _particle _gear) (break `/Game/Tools/NotedPro/NotedProFiles/Structs/SNotedProIconImage` (`self.Icon Struct`)))
  ;[1 1 1] Set Icons
  (bind _output_get (`self.Get and set note tool ref`))
  (bind _output_get_2 (set `self.Array of icons` (`|MakeArray` _note _fixit _eye _lighting _sound _player _questionmark _exclamationmark _bp _c__ _generic _geometry _texture _trash _heart _happyface _sadface _neutralface _landscape _particle _gear)))
  (set `self.New icon` (`|GetArrayItem` _output_get_2 (`KismetMathLibrary.Conv_ByteToInt` (`self.Icon Statues`))))
  (bind _icon (`/Game/Tools/NotedPro/NotedProFiles/Widget/WBP_NotedPro.Icon` _output_get))
  (bind (_imagesize _margin _tintcolor _resourceobject _drawas _tiling _mirroring) (break `SlateBrush` (`Image.Brush` _icon)))
  (`Image.SetBrush` _icon (make `SlateBrush` _imagesize _margin _tintcolor (`self.New icon`) _drawas _tiling _mirroring)))

(fn `Set note priority levels`
  (locals (`Note tool ref local` :type "/Game/Tools/NotedPro/NotedProFiles/Widget/WBP_NotedPro Object Reference"))
  ;[1 1 1] Set Note Priority Levels
  (bind _output_get (`self.Get and set note tool ref`))
  (set `local.Note tool ref local` _output_get)
  (switch `/Game/Tools/NotedPro/NotedProFiles/Enums/ENotedProPriority` (`self.Priority level`)
    (:`NewEnumerator0`
      (`Image.SetColorAndOpacity` (`/Game/Tools/NotedPro/NotedProFiles/Widget/WBP_NotedPro.NoteBackgroundColor` (`local.Note tool ref local`)) (`self.Neutral priority`))
      (`Image.SetColorAndOpacity` (`/Game/Tools/NotedPro/NotedProFiles/Widget/WBP_NotedPro.IconBG` (`local.Note tool ref local`)) (`self.Neutral priority`)))
    (:`NewEnumerator1`
      (`Image.SetColorAndOpacity` (`/Game/Tools/NotedPro/NotedProFiles/Widget/WBP_NotedPro.IconBG` (`local.Note tool ref local`)) (`self.Low priority`))
      (`Image.SetColorAndOpacity` (`/Game/Tools/NotedPro/NotedProFiles/Widget/WBP_NotedPro.NoteBackgroundColor` (`local.Note tool ref local`)) (`self.Low priority`)))
    (:`NewEnumerator2`
      (`Image.SetColorAndOpacity` (`/Game/Tools/NotedPro/NotedProFiles/Widget/WBP_NotedPro.NoteBackgroundColor` (`local.Note tool ref local`)) (`self.High priority`))
      (`Image.SetColorAndOpacity` (`/Game/Tools/NotedPro/NotedProFiles/Widget/WBP_NotedPro.IconBG` (`local.Note tool ref local`)) (`self.High priority`)))
    (:`NewEnumerator3`
      (`Image.SetColorAndOpacity` (`/Game/Tools/NotedPro/NotedProFiles/Widget/WBP_NotedPro.NoteBackgroundColor` (`local.Note tool ref local`)) (`self.Fixed`))
      (`Image.SetColorAndOpacity` (`/Game/Tools/NotedPro/NotedProFiles/Widget/WBP_NotedPro.IconBG` (`local.Note tool ref local`)) (`self.Fixed`)))))

(fn `Set note scale + position`
  (bind _returnvalue (`KismetMathLibrary.MapRangeClamped` (`self.Size of note`) 0.0 2.0 0.0 0.2))
  (`SceneComponent.SetWorldScale3D` (`self.Scene`) (1.0 1.0 1.0))
  ;[1 1 1] Sets relative Note scaling
  (`SceneComponent.SetRelativeScale3D` (`self.Widget`) (`KismetMathLibrary.Conv_DoubleToVector` _returnvalue))
  ;[1 1 1] Makes note pivot always on the bottom regardless of size
  (`SceneComponent.K2_SetRelativeLocation` (`self.Widget`) (`KismetMathLibrary.MakeVector` 0.0 0.0 (`KismetMathLibrary.Lerp` 0.0 130.0 (`KismetMathLibrary.MapRangeClamped` _returnvalue 0.0 0.2 0.0 1.0))) false false))

(fn `Set note text`
  (locals (`Note tool ref local` :type "/Game/Tools/NotedPro/NotedProFiles/Widget/WBP_NotedPro Object Reference"))
  (bind _returnvalue (`KismetTextLibrary.Conv_TextToString` (`KismetTextLibrary.Conv_StringToText` (`KismetStringLibrary.Replace` (`KismetTextLibrary.Conv_TextToString` (`self.Message`)) "  " " \n"))))
  ;[1 1 1] Set Note Text
  (bind _output_get (`self.Get and set note tool ref`))
  (set `local.Note tool ref local` _output_get)
  (`|ExecutionSequence`
    (:`then_0`
      (`TextBlock.SetText` (`/Game/Tools/NotedPro/NotedProFiles/Widget/WBP_NotedPro.NoteHeader` (`local.Note tool ref local`)) (`KismetTextLibrary.Conv_StringToText` (`KismetStringLibrary.Concat_StrStr` "- " (`KismetTextLibrary.Conv_TextToString` (`self.Header / Topic`)) " -"))))
    (:`then_1`
      (if (`|EnumEquality` (`self.Team members`) "NewEnumerator0")
        (`TextBlock.SetText` (`/Game/Tools/NotedPro/NotedProFiles/Widget/WBP_NotedPro.NoteText` (`local.Note tool ref local`)) (`KismetTextLibrary.Conv_StringToText` (`KismetStringLibrary.Concat_StrStr` "Note: " _returnvalue)))
        (else
          (`TextBlock.SetText` (`/Game/Tools/NotedPro/NotedProFiles/Widget/WBP_NotedPro.NoteText` (`local.Note tool ref local`)) (`KismetTextLibrary.Conv_StringToText` (`KismetStringLibrary.Concat_StrStr` (`|GetEnumeratorNameAsString` (`self.Team members`)) ": " _returnvalue))))))))

(fn `Sort out notes`
  (params (`Noted ref` :type "/Game/Tools/NotedPro/BP_NotedPro Object Reference"))
  (returns (`T or F` :type Boolean))
  (bind _sort_by__priority_level (`self.Sort by: Priority Level`))
  (bind _sort_by__icon_statues (`self.Sort by: Icon Statues`))
  (bind _sort_by__team_members (`self.Sort by: Team members`))
  (return (and (or (`|EnumEquality` "NewEnumerator0" _sort_by__team_members) (== (`KismetSystemLibrary.MakeLiteralByte` _sort_by__team_members) (`/Game/Tools/NotedPro/BP_NotedPro.Team members` `Noted ref`))) (or (`|EnumEquality` "NewEnumerator23" _sort_by__icon_statues) (== (- (`KismetSystemLibrary.MakeLiteralByte` _sort_by__icon_statues) 1) (`/Game/Tools/NotedPro/BP_NotedPro.Icon Statues` `Noted ref`))) (or (`|EnumEquality` "NewEnumerator4" _sort_by__priority_level) (== (- (`KismetSystemLibrary.MakeLiteralByte` _sort_by__priority_level) 1) (`/Game/Tools/NotedPro/BP_NotedPro.Priority level` `Noted ref`))))))

(fn `Tether scale`
  (bind _returnvalue (`KismetMathLibrary.Conv_DoubleToVector` (`KismetMathLibrary.Lerp` 0.2 2.0 (`KismetMathLibrary.MapRangeClamped` (`self.Size of note`) 0.2 2.0 0.0 1.0))))
  (for _array_element (`self.Tether struct`)
    (bind (_tethercableref _actorreftopointto _endpointnotetonoteonly) (break `/Game/Tools/NotedPro/NotedProFiles/Tethering/SNotedProTether` _array_element))
    (`/Engine/EditorBlueprintResources/StandardMacros.IsValid` _endpointnotetonoteonly
      (:`Is Valid`
        (`self.SetActorScale3D` _tethercableref _returnvalue))
      (:`Is Not Valid`
        (`self.SetActorScale3D` _tethercableref _returnvalue))))
  (return))

(fn `Tether system`
  (locals (`Note tool ref local` :type "/Game/Tools/NotedPro/NotedProFiles/Widget/WBP_NotedPro Object Reference"))
  (bind _spline_pointer (`self.Spline pointer`))
  (bind _point_to_actors_cleaned (`self.Point to actors cleaned`))
  (bind _output_get (`self.Get and set note tool ref`))
  (set `local.Note tool ref local` _output_get)
  ;[1 1 1] Hidden state
  (`SceneComponent.SetHiddenInGame` _spline_pointer true false)
  (`SceneComponent.SetVisibility` _spline_pointer false false)
  ;[1 1 1] Valid references only
  (`KismetArrayLibrary.Array_Clear` (`self.Point to actors cleaned`))
  (for _array_element (`self.Point to actors`)
    (`/Engine/EditorBlueprintResources/StandardMacros.IsValid` _array_element
      (:`Is Valid`
        (`KismetArrayLibrary.Array_Add` (`self.Point to actors cleaned`) _array_element))))
  ;[1 1 1] Prevents constant cable creation. If the system has what it needs in terms of calbes it stops.
  (if (and (`KismetArrayLibrary.Array_IsValidIndex` _point_to_actors_cleaned) (!= (`KismetArrayLibrary.Array_Length` (`self.Tether struct`)) (`KismetArrayLibrary.Array_Length` _point_to_actors_cleaned)))
    (`self.Create attach remove cables`)
    (else
      (`self.Cable on spline logic`))))

(fn `UserConstructionScript`
  (set `self.Game playing?` false)
  (`self.Set note scale + position`)
  (`self.Pass global note variables to party`)
  (`self.Get and set note tool ref`)
  (`PrimitiveComponent.SetRenderCustomDepth` (`self.Widget`) (`self.Render custom depth?`))
  (`PrimitiveComponent.SetCustomDepthStencilValue` (`self.Widget`) (`self.Stencil #`))
  ;[1 1 1] This is what ticks the utility to work in editor
  (`KismetSystemLibrary.K2_SetTimer` self "Utility Tick" 0.01 true))

(fn `↑ Scroll ↑`
  (bind _returnvalue (`self.Scroll Calculations -`))
  (`ScrollBox.SetScrollOffset` (`/Game/Tools/NotedPro/NotedProFiles/Widget/WBP_NotedPro.ScrollBox_main` (cast `/Game/Tools/NotedPro/NotedProFiles/Widget/WBP_NotedPro` (`WidgetComponent.GetUserWidgetObject` (`self.Widget`)) :!pure true)) _returnvalue))

(fn `↓ Scroll ↓`
  (bind _returnvalue (`self.Scroll Calculations +`))
  (`ScrollBox.SetScrollOffset` (`/Game/Tools/NotedPro/NotedProFiles/Widget/WBP_NotedPro.ScrollBox_main` (cast `/Game/Tools/NotedPro/NotedProFiles/Widget/WBP_NotedPro` (`WidgetComponent.GetUserWidgetObject` (`self.Widget`)) :!pure true)) _returnvalue)
  (bind _output_get (`self.Get and set note tool ref`))
  (bind _asvertical_box_slot (cast `VerticalBoxSlot` (`Widget.Slot` (`/Game/Tools/NotedPro/NotedProFiles/Widget/WBP_NotedPro.VerticalBox_Sub` _output_get))))
  (`VerticalBoxSlot.SetPadding` _asvertical_box_slot (make `Margin` 0.0 0.0 100.0)))