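; Tether cable actor for the NotedPro tool that visually links to a target actor in a given color.
; AttachCableFunc attaches the cable end to the target, or to its own endpoint child actor when the target is another BP_NotedPro.
; It tints the cable with a dynamic Mat_Tether instance.
; A second instance colors both its pointer mesh and the endpoint's, provided the endpoint's mesh is valid.
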(fn `Attach Cable Func`
  (params (`Actor to attach` :type "Actor Object Reference") (Color :type "LinearColor Structure"))
  (bind (_r _g _b _a) (break `LinearColor` Color))
  (bind (_r_2 _g_2 _b_2) (break `LinearColor` Color))
  (if (== (`GameplayStatics.GetObjectClass` `Actor to attach`) "/Game/Tools/NotedPro/BP_NotedPro.BP_NotedPro_C")
    (`CableComponent.SetAttachEndTo` (`self.CableComponent`) (`ChildActorComponent.ChildActor` (`self.Tether_Cable_Endpoint (NtoN)`)) "None" "None")
    (else
      (`CableComponent.SetAttachEndTo` (`self.CableComponent`) `Actor to attach` "None" "None")))
  (bind _returnvalue (`KismetMaterialLibrary.CreateDynamicMaterialInstance` "/Game/Tools/NotedPro/NotedProFiles/Tethering/Mat_Tether.Mat_Tether"))
  (`PrimitiveComponent.SetMaterial` (`self.CableComponent`) 0 _returnvalue)
  (`MaterialInstanceDynamic.SetVectorParameterValue` _returnvalue "Pointer Color" (make `LinearColor` _r_2 _g_2 _b_2 1.0))
  (bind _returnvalue_2 (`KismetMaterialLibrary.CreateDynamicMaterialInstance` "/Game/Tools/NotedPro/NotedProFiles/Tethering/Mat_Tether.Mat_Tether"))
  (`/Engine/EditorBlueprintResources/StandardMacros.IsValid` (`/Game/Tools/NotedPro/NotedProFiles/Tethering/BP_NotedPro_TetherCableEndpoint.Pointer_Mesh` (cast `/Game/Tools/NotedPro/NotedProFiles/Tethering/BP_NotedPro_TetherCableEndpoint` (`ChildActorComponent.ChildActor` (`self.Tether_Cable_Endpoint (NtoN)`)) :!pure true))
    (:`Is Valid`
      (`PrimitiveComponent.SetMaterial` (`self.Pointer_Mesh`) 0 _returnvalue_2)
      (`PrimitiveComponent.SetMaterial` (`/Game/Tools/NotedPro/NotedProFiles/Tethering/BP_NotedPro_TetherCableEndpoint.Pointer_Mesh` (cast `/Game/Tools/NotedPro/NotedProFiles/Tethering/BP_NotedPro_TetherCableEndpoint` (`ChildActorComponent.ChildActor` (`self.Tether_Cable_Endpoint (NtoN)`)) :!pure true)) 0 _returnvalue_2)
      (`MaterialInstanceDynamic.SetVectorParameterValue` _returnvalue_2 "Pointer Color" (make `LinearColor` _r _g _b _a)))))

(fn `UserConstructionScript`)